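; Actor component that gives the slicing dummy and lizard enemies physics-driven hit reactions and ragdolling.
; On BeginPlay it adds a PhysicalAnimation component and binds it to the owner's mesh.
; Hits apply a profile and impulse below the spine, adding time to a Tick-driven countdown that fades physics blend weight, then disables simulation and ticking.
; EnterRagdoll simulates from the spine down with the Ragdoll profiles and halts character movement.
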(event `self.ReceiveBeginPlay`
  (bind _returnvalue (`self.GetOwner`))
  (bind _returnvalue_2 (`|AddComponentByClass` (`self.GetOwner`) "/Script/Engine.PhysicalAnimationComponent"))
  (bind _output_get (set `self.PhysicalAnimationComponent` _returnvalue_2))
  ;[1 1 1] Temp
  ; FUTURE PARENT ACTOR
  (bind _asslicing_dummy_ai (cast `/Game/Transfusion/Blueprints/BP_Enemy/Slicing_Dummy/Slicing_Dummy_AI` _returnvalue)
    (:`then`
      (bind _mesh (`Character.Mesh` _asslicing_dummy_ai))
      (`PhysicalAnimationComponent.SetSkeletalMeshComponent` _output_get _mesh)
      (set `self.Skeletal Mesh` _mesh)
      (set `self.CapsuleComponent` (`Character.CapsuleComponent` _asslicing_dummy_ai))
      (set `self.Character Movement` (`Character.CharacterMovement` _asslicing_dummy_ai)))
    (:`CastFailed`
      (bind _asbp_lizard_enemy_base (cast `/Game/Transfusion/Blueprints/BP_Enemy/BP_LizardEnemy_Base` _returnvalue))
      (bind _mesh_2 (`Character.Mesh` _asbp_lizard_enemy_base))
      (`PhysicalAnimationComponent.SetSkeletalMeshComponent` _output_get _mesh_2)
      (set `self.Skeletal Mesh` _mesh_2)
      (set `self.CapsuleComponent` (`Character.CapsuleComponent` _asbp_lizard_enemy_base))
      (set `self.Character Movement` (`Character.CharacterMovement` _asbp_lizard_enemy_base)))))

(event `self.ReceiveTick`
  (params (DeltaSeconds :type "Float (single-precision)"))
  (if (`self.IsRagdolling`)
    (`self.SetComponentTickEnabled` false)
    (else
      (set `self.HitReactionTimeRemaining` (- (`KismetMathLibrary.FInterpTo` (`self.HitReactionTimeRemaining`) 0.0 0.0 1.0) (* DeltaSeconds 1.0)))
      (if (<= (`self.HitReactionTimeRemaining`) 0.0)
        (set `self.HitReactionTimeRemaining` 0.0)
        ;[1 1 1] Causes warnings
        (`SkeletalMeshComponent.SetAllBodiesBelowSimulatePhysics` (`self.Skeletal Mesh`) "spine" false true)
        (`self.SetComponentTickEnabled` false)
        (else
          (`SkeletalMeshComponent.SetAllBodiesBelowPhysicsBlendWeight` (`self.Skeletal Mesh`) "spine" (`KismetMathLibrary.FMin` (`self.HitReactionTimeRemaining`) 1.0) false true))))))

(event `EnterRagdoll`
  (set `self.IsRagdolling` true)
  (`SkeletalMeshComponent.SetAllBodiesBelowPhysicsBlendWeight` (`self.Skeletal Mesh`) "spine" 0.0 false true)
  (`SkeletalMeshComponent.SetAllBodiesBelowSimulatePhysics` (`self.Skeletal Mesh`) "spine" true true)
  (`PhysicalAnimationComponent.ApplyPhysicalAnimationProfileBelow` (`self.PhysicalAnimationComponent`) "spine" "Ragdoll" true true)
  (`CharacterMovementComponent.SetMovementMode` (`self.Character Movement`) "MOVE_None" 0)
  ;[1 1 1] Need to Test
  (`PrimitiveComponent.SetCollisionProfileName` (`self.Skeletal Mesh`) "Ragdoll" false)
  (set `self.HitReactionTimeRemaining` 0.0)
  (`KismetSystemLibrary.PrintString` "Toggled Ragdoll"))

(event `HitReaction`
  (params (Hit :type "HitResult Structure") (`Hit Velocity` :type "Float (double-precision)"))
  (bind (_bblockinghit _binitialoverlap _time _distance _location _impactpoint _normal _impactnormal _physmat _hitactor _hitcomponent _hitbonename _hititem _elementindex _faceindex _tracestart _traceend) (`GameplayStatics.BreakHitResult` Hit))
  (`self.SetComponentTickEnabled` true)
  (set `self.HitReactionTimeRemaining` (+ (`self.HitReactionTimeRemaining`) 0.25))
  (`PhysicalAnimationComponent.ApplyPhysicalAnimationProfileBelow` (`self.PhysicalAnimationComponent`) "spine" "HitReaction" false false)
  (`SkeletalMeshComponent.SetAllBodiesBelowSimulatePhysics` (`self.Skeletal Mesh`) "spine" true false)
  (`PrimitiveComponent.AddImpulse` (`self.Skeletal Mesh`) (* (`KismetMathLibrary.Normal` (- _traceend _tracestart)) (/ `Hit Velocity` 200.0)) (select `bool` (== _hitbonename "spine") :`false` _hitbonename :`true` "spine_001") false))

(fn `ResetPhysicalAnimation`
  (set `self.HitReactionTimeRemaining` 0.0)
  (`SkeletalMeshComponent.SetAllBodiesBelowPhysicsBlendWeight` (`self.Skeletal Mesh`) "spine" 0.0 false true))