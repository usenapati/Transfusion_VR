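; VR physics grab item that the player holds through the left or right physics handle on VRPawn_Main.
; GrabComponent events drive grab and release, snapping the hand mesh onto the item's grip socket and restoring it afterward.
; While held, Tick steers the handle toward the motion controller and hits play speed-scaled haptics.
; A fast enough release flags the item airborne and adds spin, cleared on hit or regrab.
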(event `self.ReceiveTick`
  (params (DeltaSeconds :type "Float (single-precision)"))
  (if (`/Game/UnrealBaseContent/VRTemplate/Blueprints/GrabComponent.bIsHeld` (`self.GrabComponent`))
    (`self.UpdatePhysicsHandle`)))

(event `self.GrabComponent.OnGrabbed`
  (`self.GrabObject`))

(event `self.GrabComponent.OnDropped`
  (`self.ReleaseObject`))

(event `self.ObjectMesh.OnComponentHit`
  (params (HitComponent :type "PrimitiveComponent Object Reference") (OtherActor :type "Actor Object Reference") (OtherComp :type "PrimitiveComponent Object Reference") (NormalImpulse :type "Vector Structure") (Hit :type "HitResult Structure (by ref)"))
  (`|ExecutionSequence`
    (:`then_0`
      (if (`self.isAirborn`)
        (`self.ToggleAirborn` false)))
    (:`then_1`
      (if (`/Game/UnrealBaseContent/VRTemplate/Blueprints/GrabComponent.bIsHeld` (`self.GrabComponent`))
        (bind _returnvalue (`PrimitiveComponent.GetPhysicsLinearVelocity` HitComponent "None"))
        (`self.DoHapticEffect` (/ (`KismetMathLibrary.VSize` _returnvalue) 100.0))))))

(fn `GrabObject`
  (bind _objectmesh (`self.ObjectMesh`))
  (bind _returnvalue (`SceneComponent.GetSocketLocation` _objectmesh "GrabHandle"))
  (bind _returnvalue_2 (`SceneComponent.K2_GetComponentRotation` _objectmesh))
  (bind _motioncontrollerref (`/Game/UnrealBaseContent/VRTemplate/Blueprints/GrabComponent.MotionControllerRef` (`self.GrabComponent`)))
  (bind _motioncontrollerref_2 (`/Game/UnrealBaseContent/VRTemplate/Blueprints/GrabComponent.MotionControllerRef` (`self.GrabComponent`)))
  (if (`KismetSystemLibrary.IsValid` (`self.HandCompRef`))
    (`self.ReleaseObject`))
  (`PrimitiveComponent.SetEnableGravity` (`self.ObjectMesh`) false)
  (set `self.LastMotionController` _motioncontrollerref)
  (bind _asvrpawn_main (cast `/Game/Transfusion/Blueprints/VRPawn_Main` (`ActorComponent.GetOwner` _motioncontrollerref)))
  (if (== (`MotionControllerComponent.MotionSource` _motioncontrollerref) "LEFT")
    ;[1 1 1] Left Hand Logic
    (`PhysicsHandleComponent.GrabComponentAtLocationWithRotation` (`/Game/Transfusion/Blueprints/VRPawn_Main.PhysicsHandleLeft` _asvrpawn_main) (`self.ObjectMesh`) "None" _returnvalue _returnvalue_2)
    (set `self.HandParentRef` _motioncontrollerref_2)
    (bind _output_get (set `self.HandCompRef` (`/Game/Transfusion/Blueprints/VRPawn_Main.HandLeft` _asvrpawn_main)))
    (set `self.HandTransformRef` (`SceneComponent.GetRelativeTransform` _output_get))
    (`SceneComponent.K2_AttachToComponent` _output_get (`self.ObjectMesh`) "GrabHandleLeft" "SnapToTarget" "SnapToTarget" "KeepWorld" true)
    (bind _output_get_2 (set `/Game/Transfusion/Blueprints/VRPawn_Main.LastHeldLeft` (`self.ObjectMesh`) _asvrpawn_main))
    (if (== _output_get_2 (`/Game/Transfusion/Blueprints/VRPawn_Main.LastHeldRight` _asvrpawn_main))
      (set `/Game/Transfusion/Blueprints/VRPawn_Main.LastHeldRight` null _asvrpawn_main))
    (else
      ;[1 1 1] Right Hand Logic
      (`PhysicsHandleComponent.GrabComponentAtLocationWithRotation` (`/Game/Transfusion/Blueprints/VRPawn_Main.PhysicsHandleRight` _asvrpawn_main) (`self.ObjectMesh`) "None" _returnvalue _returnvalue_2)
      (set `self.HandParentRef` _motioncontrollerref_2)
      (bind _output_get_3 (set `self.HandCompRef` (`/Game/Transfusion/Blueprints/VRPawn_Main.HandRight` _asvrpawn_main)))
      (set `self.HandTransformRef` (`SceneComponent.GetRelativeTransform` _output_get_3))
      (`SceneComponent.K2_AttachToComponent` _output_get_3 (`self.ObjectMesh`) "GrabHandle" "SnapToTarget" "SnapToTarget" "KeepWorld" true)
      (bind _output_get_4 (set `/Game/Transfusion/Blueprints/VRPawn_Main.LastHeldRight` (`self.ObjectMesh`) _asvrpawn_main))
      (if (== _output_get_4 (`/Game/Transfusion/Blueprints/VRPawn_Main.LastHeldLeft` _asvrpawn_main))
        (set `/Game/Transfusion/Blueprints/VRPawn_Main.LastHeldLeft` null _asvrpawn_main))))
  (if (`self.isAirborn`)
    (`self.ToggleAirborn` false)
    (`KismetSystemLibrary.PrintString` "Grabbed")))

(fn `ReleaseObject`
  (locals (AirbornTriggerSpeed :type "Float (double-precision)" :default 400000.0))
  (bind _handcompref (`self.HandCompRef`))
  (bind _motioncontrollerref (`/Game/UnrealBaseContent/VRTemplate/Blueprints/GrabComponent.MotionControllerRef` (`self.GrabComponent`)))
  (`|ExecutionSequence`
    (:`then_0`
      (set `self.LastMotionController` _motioncontrollerref)
      (`PrimitiveComponent.SetEnableGravity` (`self.ObjectMesh`) true)
      (bind _asvrpawn_main (cast `/Game/Transfusion/Blueprints/VRPawn_Main` (`ActorComponent.GetOwner` _motioncontrollerref)))
      (if (== (`MotionControllerComponent.MotionSource` (`self.HandParentRef`)) "LEFT")
        ;[1 1 1] Left Hand Release
        (`PhysicsHandleComponent.ReleaseComponent` (`/Game/Transfusion/Blueprints/VRPawn_Main.PhysicsHandleLeft` _asvrpawn_main))
        (else
          ;[1 1 1] Right Hand Release
          (`PhysicsHandleComponent.ReleaseComponent` (`/Game/Transfusion/Blueprints/VRPawn_Main.PhysicsHandleRight` _asvrpawn_main))))
      (`SceneComponent.K2_AttachToComponent` _handcompref (`self.HandParentRef`) "None" "SnapToTarget" "SnapToTarget" "SnapToTarget" true)
      (`SceneComponent.K2_SetRelativeTransform` _handcompref (`self.HandTransformRef`) false false)
      (set `self.HandCompRef` null)
      (set `self.HandParentRef` null)
      (set `self.HandTransformRef` (struct))
      (`KismetSystemLibrary.PrintString` "Released"))
    (:`then_1`
      (bind _returnvalue (`PrimitiveComponent.GetPhysicsLinearVelocity` (`self.ObjectMesh`) "None"))
      (if (>= (`KismetMathLibrary.VSizeSquared` _returnvalue) (`local.AirbornTriggerSpeed`))
        (`self.ToggleAirborn` true)))))

(fn `ToggleAirborn`
  (params (Airborn :type Boolean))
  (returns (IsAirborn :type Boolean))
  (locals (SpinSpeed :type "Float (double-precision)" :default 50000.0))
  (bind _objectmesh (`self.ObjectMesh`))
  (bind _output_get (set `self.isAirborn` Airborn))
  (if _output_get
    (`PrimitiveComponent.SetPhysicsAngularVelocityInDegrees` _objectmesh (* (`SceneComponent.GetRightVector` _objectmesh) (`local.SpinSpeed`)) true "None")
    (return (`self.isAirborn`))
    (else
      (`KismetSystemLibrary.PrintString` "Hello" true true (struct :`R` 1.0 :`G` 0.784709 :`A` 1.0)))))

(fn `UpdatePhysicsHandle`
  (bind _grabcomponent (`self.GrabComponent`))
  (bind _motioncontrollerref (`/Game/UnrealBaseContent/VRTemplate/Blueprints/GrabComponent.MotionControllerRef` _grabcomponent))
  (bind _returnvalue (`SceneComponent.K2_GetComponentLocation` _motioncontrollerref))
  (bind _returnvalue_2 (`KismetMathLibrary.ComposeRotators` (`KismetMathLibrary.NegateRotator` (`SceneComponent.RelativeRotation` _grabcomponent)) (`SceneComponent.K2_GetComponentRotation` _motioncontrollerref)))
  (bind _asvrpawn_main (cast `/Game/Transfusion/Blueprints/VRPawn_Main` (`ActorComponent.GetOwner` (`/Game/UnrealBaseContent/VRTemplate/Blueprints/GrabComponent.MotionControllerRef` (`self.GrabComponent`)))))
  (if (== (`MotionControllerComponent.MotionSource` (`self.HandParentRef`)) "LEFT")
    ;[1 1 1] Left Hand Update
    (`PhysicsHandleComponent.SetTargetLocationAndRotation` (`/Game/Transfusion/Blueprints/VRPawn_Main.PhysicsHandleLeft` _asvrpawn_main) _returnvalue _returnvalue_2)
    (else
      ;[1 1 1] Right Hand Update
      (`PhysicsHandleComponent.SetTargetLocationAndRotation` (`/Game/Transfusion/Blueprints/VRPawn_Main.PhysicsHandleRight` _asvrpawn_main) _returnvalue _returnvalue_2))))

(fn `UserConstructionScript`)