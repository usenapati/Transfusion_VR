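; CircleSlider is a player interactible whose Slider component is dragged along a spline by a motion controller.
; Grabbing through the GrabComponent stores the controller reference, and dropping clears it if that same controller is still stored.
; While the reference is valid, Tick sweeps the Slider to the spline point at the input key closest to the controller, keeping it constrained to the path.
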(event `self.ReceiveTick`
  (params (DeltaSeconds :type "Float (single-precision)"))
  (bind _spline (`self.Spline`))
  (bind _motion_controller_ref (`self.Motion Controller Ref`))
  (`/Engine/EditorBlueprintResources/StandardMacros.IsValid` _motion_controller_ref
    (:`Is Valid`
      (`SceneComponent.K2_SetWorldLocation` (`self.Slider`) (`SplineComponent.GetLocationAtSplineInputKey` _spline (`SplineComponent.FindInputKeyClosestToWorldLocation` _spline (`SceneComponent.K2_GetComponentLocation` _motion_controller_ref)) "World") true false))))

(event `self.GrabComponent.OnGrabbed`
  (set `self.Motion Controller Ref` (`/Game/UnrealBaseContent/VRTemplate/Blueprints/GrabComponent.MotionControllerRef` (`self.GrabComponent`))))

(event `self.GrabComponent.OnDropped`
  (if (== (`/Game/UnrealBaseContent/VRTemplate/Blueprints/GrabComponent.MotionControllerRef` (`self.GrabComponent`)) (`self.Motion Controller Ref`))
    (set `self.Motion Controller Ref` null)))

(fn `UserConstructionScript`)