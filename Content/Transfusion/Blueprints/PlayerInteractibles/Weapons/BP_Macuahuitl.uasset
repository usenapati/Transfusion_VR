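; BP_Macuahuitl is a grabbable VR sword with a magic ability that temporarily turns it into a bigger, stronger blade.
; UseMagic doubles scale, damage and trail width, lowers the swing threshold and changes the holding hand's physics handle interpolation speed until a timer calls ResetBigSword.
; A dynamic material lights the blade while magic is active.
; Going airborne adds spin and swaps collision settings, and the first grab notifies the tutorial.
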(fn `GrabObject`
  (`parent.GrabObject`)
  (`/Engine/EditorBlueprintResources/StandardMacros.DoOnce` false
    (:`Completed`
      (bind _asvrpawn_main (cast `/Game/Transfusion/Blueprints/VRPawn_Main` (`GameplayStatics.GetPlayerPawn` 0)))
      (`/Game/Transfusion/Blueprints/VRPawn_Main.NotifyTutorial` _asvrpawn_main false false false true false false))))

(fn `ResetBigSword`
  (locals (NormalSwordSpeed :type "Float (double-precision)" :default 25.0))
  (bind _objectmesh (`self.ObjectMesh`))
  (bind _normalswordspeed (`local.NormalSwordSpeed`))
  (bind _lastmotioncontroller (`self.LastMotionController`))
  (`SceneComponent.SetWorldScale3D` _objectmesh (/ (`SceneComponent.K2_GetComponentScale` _objectmesh) 2.0))
  (bind _asvrpawn_main (cast `/Game/Transfusion/Blueprints/VRPawn_Main` (`ActorComponent.GetOwner` _lastmotioncontroller)))
  (if (== (`MotionControllerComponent.MotionSource` _lastmotioncontroller) "LEFT")
    (`PhysicsHandleComponent.SetInterpolationSpeed` (`/Game/Transfusion/Blueprints/VRPawn_Main.PhysicsHandleLeft` _asvrpawn_main) _normalswordspeed)
    (else
      (`PhysicsHandleComponent.SetInterpolationSpeed` (`/Game/Transfusion/Blueprints/VRPawn_Main.PhysicsHandleRight` _asvrpawn_main) _normalswordspeed)))
  (set `self.RequiredSwingVelocity` (* (`self.RequiredSwingVelocity`) 4.0))
  (set `self.BodyDamage` (/ (`self.BodyDamage`) 2))
  (set `self.JointDamage` (/ (`self.JointDamage`) 2))
  (`FXSystemComponent.SetFloatParameter` (`self.SwordTrail`) "TrailWidth" (`self.SwordLength`))
  (set `self.MagicBlocked` false)
  (set `self.UsingMagic` false))

(fn `ToggleAirborn`
  (params (Airborn :type Boolean))
  (returns (IsAirborn :type Boolean))
  (locals (SpinSpeed :type "Float (double-precision)" :default 30000.0))
  (bind _objectmesh (`self.ObjectMesh`))
  (bind _objectmesh_2 (`self.ObjectMesh`))
  (bind _objectmesh_3 (`self.ObjectMesh`))
  (bind _output_get (set `self.isAirborn` Airborn))
  (if _output_get
    (`PrimitiveComponent.SetPhysicsAngularVelocityInDegrees` _objectmesh_2 (* (`SceneComponent.GetRightVector` _objectmesh_2) (`local.SpinSpeed`)) true "None")
    (`PrimitiveComponent.SetCollisionObjectType` _objectmesh_3 "ECC_GameTraceChannel2")
    (`PrimitiveComponent.SetCollisionResponseToChannel` _objectmesh_3 "ECC_WorldDynamic" "ECR_Overlap")
    (`PrimitiveComponent.SetCollisionEnabled` (`self.SlashPlane`) "NoCollision")
    (`PrimitiveComponent.SetCollisionEnabled` (`self.StabPlane`) "NoCollision")
    (else
      (`PrimitiveComponent.SetCollisionObjectType` _objectmesh "ECC_PhysicsBody")
      (`PrimitiveComponent.SetCollisionResponseToChannel` _objectmesh "ECC_WorldDynamic" "ECR_Block")
      (`PrimitiveComponent.SetCollisionEnabled` (`self.SlashPlane`) "QueryOnly")
      (`PrimitiveComponent.SetCollisionEnabled` (`self.StabPlane`) "QueryOnly")))
  (return (`local.Airborn`)))

(fn `ToggleMagicActive`
  (params (Active :type Boolean))
  (bind _swordmaterial (`self.SwordMaterial`))
  (`parent.ToggleMagicActive` Active)
  (if Active
    (`MaterialInstanceDynamic.SetScalarParameterValue` _swordmaterial "BladeLightIntensity" 2.0)
    (else
      (`MaterialInstanceDynamic.SetScalarParameterValue` _swordmaterial "BladeLightIntensity" 0.0))))

(fn `UseMagic`
  (locals (BigSwordDuration :type "Float (double-precision)" :default 10.0) (SlowSwordSpeed :type "Float (double-precision)" :default 12.0))
  (bind _objectmesh (`self.ObjectMesh`))
  (bind _slowswordspeed (`local.SlowSwordSpeed`))
  (bind _lastmotioncontroller (`self.LastMotionController`))
  (bind _use_magic_ (`parent.UseMagic`))
  (if _use_magic_
    (`SceneComponent.SetWorldScale3D` _objectmesh (* (`SceneComponent.K2_GetComponentScale` _objectmesh) 2.0))
    (bind _asvrpawn_main (cast `/Game/Transfusion/Blueprints/VRPawn_Main` (`ActorComponent.GetOwner` _lastmotioncontroller)))
    (if (== (`MotionControllerComponent.MotionSource` _lastmotioncontroller) "LEFT")
      (`PhysicsHandleComponent.SetInterpolationSpeed` (`/Game/Transfusion/Blueprints/VRPawn_Main.PhysicsHandleLeft` _asvrpawn_main) _slowswordspeed)
      (else
        (`PhysicsHandleComponent.SetInterpolationSpeed` (`/Game/Transfusion/Blueprints/VRPawn_Main.PhysicsHandleRight` _asvrpawn_main) _slowswordspeed)))
    (set `self.RequiredSwingVelocity` (/ (`self.RequiredSwingVelocity`) 4.0))
    (set `self.BodyDamage` (* (`self.BodyDamage`) 2))
    (set `self.JointDamage` (* (`self.JointDamage`) 2))
    (`FXSystemComponent.SetFloatParameter` (`self.SwordTrail`) "TrailWidth" (* (`self.SwordLength`) 2.0))
    (set `self.MagicBlocked` true)
    (`KismetSystemLibrary.K2_SetTimer` null "ResetBigSword" (`local.BigSwordDuration`))))

(fn `UserConstructionScript`
  (`parent.UserConstructionScript`)
  (bind _returnvalue (`PrimitiveComponent.CreateDynamicMaterialInstance` (`self.ObjectMesh`) 0 null "None"))
  (set `self.SwordMaterial` _returnvalue))