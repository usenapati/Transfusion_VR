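; VR short sword weapon whose magic fires a lightning beam along the blade.
; UseMagic line-traces from the blade socket, applies a timed freeze status through IStatusInterface, then chains to pawns within a sphere around the hit, drawing Niagara beams.
; ToggleAirborn spins the thrown sword and swaps its collision, disabling slash and stab planes in flight.
; A dynamic material lights the blade while magic is active; older time-slow magic remains as unreachable, deprecated nodes.
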(fn `ToggleAirborn`
  (params (Airborn :type Boolean))
  (returns (IsAirborn :type Boolean))
  (locals (SpinSpeed :type "Float (double-precision)" :default 30000.0))
  (bind _objectmesh (`self.ObjectMesh`))
  (bind _objectmesh_2 (`self.ObjectMesh`))
  (bind _objectmesh_3 (`self.ObjectMesh`))
  (bind _output_get (set `self.isAirborn` Airborn))
  (if _output_get
    (`PrimitiveComponent.SetPhysicsAngularVelocityInDegrees` _objectmesh_2 (* (`SceneComponent.GetRightVector` _objectmesh_2) (`local.SpinSpeed`)) true "None")
    (`PrimitiveComponent.SetCollisionObjectType` _objectmesh_3 "ECC_GameTraceChannel2")
    (`PrimitiveComponent.SetCollisionResponseToChannel` _objectmesh_3 "ECC_WorldDynamic" "ECR_Overlap")
    (`PrimitiveComponent.SetCollisionEnabled` (`self.SlashPlane`) "NoCollision")
    (`PrimitiveComponent.SetCollisionEnabled` (`self.StabPlane`) "NoCollision")
    (else
      (`PrimitiveComponent.SetCollisionObjectType` _objectmesh "ECC_PhysicsBody")
      (`PrimitiveComponent.SetCollisionResponseToChannel` _objectmesh "ECC_WorldDynamic" "ECR_Block")
      (`PrimitiveComponent.SetCollisionEnabled` (`self.SlashPlane`) "QueryOnly")
      (`PrimitiveComponent.SetCollisionEnabled` (`self.StabPlane`) "QueryOnly")))
  (return (`local.Airborn`)))

(fn `ToggleMagicActive`
  (params (Active :type Boolean))
  (bind _swordmaterial (`self.SwordMaterial`))
  (`parent.ToggleMagicActive` Active)
  (if Active
    (`MaterialInstanceDynamic.SetScalarParameterValue` _swordmaterial "BladeLightIntensity" 2.0)
    (else
      (`MaterialInstanceDynamic.SetScalarParameterValue` _swordmaterial "BladeLightIntensity" 0.0))))

(fn `UseMagic`
  (locals (TimeSlowLength :type "Float (double-precision)" :default 5.0) (ChainSphereRadius :type "Float (double-precision)" :default 500.0) (LightningLength :type "Float (double-precision)" :default 500.0))
  (bind (_returnvalue_location _returnvalue_rotation) (`KismetMathLibrary.BreakTransform` (`SceneComponent.GetSocketTransform` (`self.ObjectMesh`) "Collision_start" "RTS_World")))
  (bind _returnvalue (+ _returnvalue_location (* (`KismetMathLibrary.GetUpVector` _returnvalue_rotation) (`local.LightningLength`))))
  (bind _use_magic_ (`parent.UseMagic`))
  (if _use_magic_
    (bind (_outhit _returnvalue_2) (`KismetSystemLibrary.LineTraceSingle` _returnvalue_location _returnvalue "TraceTypeQuery1"))
    (if _returnvalue_2
      ;[1 1 1] Spawn a lightning particle regardless of whether we hit an enemy or not
      (bind _returnvalue_3 (`NiagaraFunctionLibrary.SpawnSystemAtLocation` "/Game/Transfusion/VFX/PS_Lightning.PS_Lightning" _returnvalue_location (struct) (1.0 1.0 1.0) true false))
      (`NiagaraComponent.SetVariableVec3` _returnvalue_3 "BeamEndPos" (`.Location` (`GameplayStatics.BreakHitResult` _outhit)))
      (`ActorComponent.Activate` _returnvalue_3 false)
      ;[1 1 1] If hit a target, freeze and chain out to more enemies
      (if (`KismetSystemLibrary.DoesImplementInterface` (`.HitActor` (`GameplayStatics.BreakHitResult` _outhit)) "/Game/Transfusion/Blueprints/Interfaces/IStatusInterface.IStatusInterface_C")
        (message `/Game/Transfusion/Blueprints/Interfaces/IStatusInterface.Enter Status Effect` (`.HitActor` (`GameplayStatics.BreakHitResult` _outhit)) "NewEnumerator0" 3.0)
        (bind _outactors (`KismetSystemLibrary.SphereOverlapActors` (`.Location` (`GameplayStatics.BreakHitResult` _outhit)) (`local.ChainSphereRadius`) (`|MakeArray` "ObjectTypeQuery3" :!type "EObjectTypeQuery Enum") null (`|MakeArray` (`GameplayStatics.GetPlayerPawn` 0) :!type "Actor Object Reference")))
        (for _array_element _outactors
          (if (`KismetSystemLibrary.DoesImplementInterface` _array_element "/Game/Transfusion/Blueprints/Interfaces/IStatusInterface.IStatusInterface_C")
            (message `/Game/Transfusion/Blueprints/Interfaces/IStatusInterface.Enter Status Effect` _array_element "NewEnumerator0" 3.0)
            (bind _returnvalue_4 (`NiagaraFunctionLibrary.SpawnSystemAtLocation` "/Game/Transfusion/VFX/PS_Lightning.PS_Lightning" (`.Location` (`GameplayStatics.BreakHitResult` _outhit)) (struct) (1.0 1.0 1.0) true false))
            (`NiagaraComponent.SetVariableVec3` _returnvalue_4 "BeamEndPos" (`self.K2_GetActorLocation` _array_element))
            (`ActorComponent.Activate` _returnvalue_4 false)))
        (set `self.MagicBlocked` false)
        (set `self.UsingMagic` false))
      (else
        ;[1 1 1] Missed everything
        (bind _returnvalue_5 (`NiagaraFunctionLibrary.SpawnSystemAtLocation` "/Game/Transfusion/VFX/PS_Lightning.PS_Lightning" _returnvalue_location (struct) (1.0 1.0 1.0) true false))
        (`NiagaraComponent.SetVariableVec3` _returnvalue_5 "BeamEndPos" _returnvalue)
        (`ActorComponent.Activate` _returnvalue_5 false)
        (set `self.MagicBlocked` false)
        (set `self.UsingMagic` false)))))

(fn `UserConstructionScript`
  (`parent.UserConstructionScript`)
  (bind _returnvalue (`PrimitiveComponent.CreateDynamicMaterialInstance` (`self.ObjectMesh`) 0 null "None"))
  (set `self.SwordMaterial` _returnvalue))