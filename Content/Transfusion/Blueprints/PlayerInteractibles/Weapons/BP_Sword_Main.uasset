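; Main VR sword weapon that spins when airborne and has a time-slowing magic ability.
; ToggleAirborn adds spin, switches collision type and WorldDynamic response, and disables the slash and stab planes until landing.
; UseMagic halves global time while speeding up the player pawn and held items to compensate, then a timer resets dilation and unblocks magic.
; A dynamic material instance made at construction lights the blade while magic is active.
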(fn `ResetTimeDilation`
  (`GameplayStatics.SetGlobalTimeDilation` 1.0)
  (bind _asvrpawn_main (cast `/Game/Transfusion/Blueprints/VRPawn_Main` (`GameplayStatics.GetPlayerPawn` 0)))
  (bind _output_get (set `Actor.CustomTimeDilation` 1.0 _asvrpawn_main))
  (bind _heldcomponentleft (`/Game/Transfusion/Blueprints/VRPawn_Main.HeldComponentLeft` _asvrpawn_main))
  (`/Engine/EditorBlueprintResources/StandardMacros.IsValid` _heldcomponentleft
    (:`Is Valid`
      (bind _output_get_2 (set `Actor.CustomTimeDilation` _output_get (`ActorComponent.GetOwner` _heldcomponentleft)))
      (bind _heldcomponentright (`/Game/Transfusion/Blueprints/VRPawn_Main.HeldComponentRight` _asvrpawn_main))
      (set `Actor.CustomTimeDilation` _output_get_2 (`ActorComponent.GetOwner` _heldcomponentright) :!label _label))
    (:`Is Not Valid`
      (`/Engine/EditorBlueprintResources/StandardMacros.IsValid` _heldcomponentright
        (:`Is Valid`
          (goto _label))
        (:`Is Not Valid`
          _))))
  (set `self.MagicBlocked` false)
  (set `self.UsingMagic` false))

(fn `ToggleAirborn`
  (params (Airborn :type Boolean))
  (returns (IsAirborn :type Boolean))
  (locals (SpinSpeed :type "Float (double-precision)" :default 30000.0))
  (bind _objectmesh (`self.ObjectMesh`))
  (bind _objectmesh_2 (`self.ObjectMesh`))
  (bind _objectmesh_3 (`self.ObjectMesh`))
  (bind _output_get (set `self.isAirborn` Airborn))
  (if _output_get
    (`PrimitiveComponent.SetPhysicsAngularVelocityInDegrees` _objectmesh_2 (* (`SceneComponent.GetRightVector` _objectmesh_2) (`local.SpinSpeed`)) true "None")
    (`PrimitiveComponent.SetCollisionObjectType` _objectmesh_3 "ECC_GameTraceChannel2")
    (`PrimitiveComponent.SetCollisionResponseToChannel` _objectmesh_3 "ECC_WorldDynamic" "ECR_Overlap")
    (`PrimitiveComponent.SetCollisionEnabled` (`self.SlashPlane`) "NoCollision")
    (`PrimitiveComponent.SetCollisionEnabled` (`self.StabPlane`) "NoCollision")
    (else
      (`PrimitiveComponent.SetCollisionObjectType` _objectmesh "ECC_PhysicsBody")
      (`PrimitiveComponent.SetCollisionResponseToChannel` _objectmesh "ECC_WorldDynamic" "ECR_Block")
      (`PrimitiveComponent.SetCollisionEnabled` (`self.SlashPlane`) "QueryOnly")
      (`PrimitiveComponent.SetCollisionEnabled` (`self.StabPlane`) "QueryOnly")))
  (return (`local.Airborn`)))

(fn `ToggleMagicActive`
  (params (Active :type Boolean))
  (bind _swordmaterial (`self.SwordMaterial`))
  (`parent.ToggleMagicActive` Active)
  (if Active
    (`MaterialInstanceDynamic.SetScalarParameterValue` _swordmaterial "BladeLightIntensity" 2.0)
    (else
      (`MaterialInstanceDynamic.SetScalarParameterValue` _swordmaterial "BladeLightIntensity" 0.0))))

(fn `UseMagic`
  (locals (TimeSlowLength :type "Float (double-precision)" :default 5.0))
  (if (== (`GameplayStatics.GetGlobalTimeDilation`) 1.0)
    (bind _use_magic_ (`parent.UseMagic`))
    (if _use_magic_
      (`GameplayStatics.SetGlobalTimeDilation` 0.5)
      (bind _asvrpawn_main (cast `/Game/Transfusion/Blueprints/VRPawn_Main` (`GameplayStatics.GetPlayerPawn` 0)))
      (bind _output_get (set `Actor.CustomTimeDilation` 2.0 _asvrpawn_main))
      (bind _heldcomponentleft (`/Game/Transfusion/Blueprints/VRPawn_Main.HeldComponentLeft` _asvrpawn_main))
      (`/Engine/EditorBlueprintResources/StandardMacros.IsValid` _heldcomponentleft
        (:`Is Valid`
          (bind _output_get_2 (set `Actor.CustomTimeDilation` _output_get (`ActorComponent.GetOwner` _heldcomponentleft))))
        (:`Is Not Valid`
          _))
      (bind _heldcomponentright (`/Game/Transfusion/Blueprints/VRPawn_Main.HeldComponentRight` _asvrpawn_main))
      (`/Engine/EditorBlueprintResources/StandardMacros.IsValid` _heldcomponentright
        (:`Is Valid`
          (set `Actor.CustomTimeDilation` _output_get_2 (`ActorComponent.GetOwner` _heldcomponentright)))
        (:`Is Not Valid`
          _))
      (set `self.MagicBlocked` true)
      (`KismetSystemLibrary.K2_SetTimer` null "ResetTimeDilation" (`local.TimeSlowLength`)))))

(fn `UserConstructionScript`
  (`parent.UserConstructionScript`)
  (bind _returnvalue (`PrimitiveComponent.CreateDynamicMaterialInstance` (`self.ObjectMesh`) 0 null "None"))
  (set `self.SwordMaterial` _returnvalue))