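; BP_PauseSphere is a VR interactable that calls TogglePause(true) on the main VR pawn when it leaves the sphere's overlap.
; It also hosts a grabbable settings wheel: grabbing attaches it to a physics handle, whose target follows the motion controller every tick until release.
; Initial wheel yaw and look-at yaw are stored on grab but never read here, and the widget's cursor-over event is empty.
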(event `self.ReceiveBeginPlay`)

(event `self.PauseSphere.OnComponentEndOverlap`
  (params (OverlappedComponent :type "PrimitiveComponent Object Reference") (OtherActor :type "Actor Object Reference") (OtherComp :type "PrimitiveComponent Object Reference") (OtherBodyIndex :type Integer))
  (bind _asvrpawn_main (cast `/Game/Transfusion/Blueprints/VRPawn_Main` OtherActor))
  (`/Game/Transfusion/Blueprints/VRPawn_Main.TogglePause` _asvrpawn_main true))

(event `self.ReceiveTick`
  (params (DeltaSeconds :type "Float (single-precision)"))
  (bind _motion_controller_ref (`self.Motion Controller Ref`))
  (`/Engine/EditorBlueprintResources/StandardMacros.IsValid` _motion_controller_ref
    (:`Is Valid`
      (`PhysicsHandleComponent.SetTargetLocation` (`self.PhysicsHandle`) (`SceneComponent.K2_GetComponentLocation` _motion_controller_ref)))))

(event `self.WheelGrabComponent.OnGrabbed`
  (bind (_returnvalue_roll _returnvalue_pitch _returnvalue_yaw) (`KismetMathLibrary.BreakRotator` (`SceneComponent.K2_GetComponentRotation` (`self.SettingsWheel`))))
  (bind _returnvalue (`SceneComponent.K2_GetComponentLocation` (`self.Motion Controller Ref`)))
  (bind (_returnvalue_roll_2 _returnvalue_pitch_2 _returnvalue_yaw_2) (`KismetMathLibrary.BreakRotator` (`KismetMathLibrary.FindLookAtRotation` (`SceneComponent.K2_GetComponentLocation` (`self.WheelGrabComponent`)) _returnvalue)))
  (set `self.Motion Controller Ref` (`/Game/UnrealBaseContent/VRTemplate/Blueprints/GrabComponent.MotionControllerRef` (`self.WheelGrabComponent`)))
  (set `self.Initial Relative Rotation Z (Yaw)` _returnvalue_yaw)
  (set `self.Initial Look At Rotation (Z)` _returnvalue_yaw_2)
  (bind _output_get (set `self.Initial Location` _returnvalue))
  (`PhysicsHandleComponent.GrabComponentAtLocation` (`self.PhysicsHandle`) (`self.SettingsWheel`) "None" _output_get))

(event `self.WheelGrabComponent.OnDropped`
  (if (== (`/Game/UnrealBaseContent/VRTemplate/Blueprints/GrabComponent.MotionControllerRef` (`self.WheelGrabComponent`)) (`self.Motion Controller Ref`))
    (set `self.Motion Controller Ref` null)
    (`PhysicsHandleComponent.ReleaseComponent` (`self.PhysicsHandle`))))

(event `self.Widget.OnBeginCursorOver`
  (params (TouchedComponent :type "PrimitiveComponent Object Reference")))

(fn `UserConstructionScript`)