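; BP_LevelCube is a sliceable level-select cube that shows a level name and opens that level after it is sliced.
; The construction script copies the static Cube into a procedural mesh with collision and writes LevelName to a text render.
; BeforeSlice starts a timer that calls LoadLevel after a delay, while GetSliceMat supplies the slice material.
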(event `/Game/Transfusion/Blueprints/Interfaces/IProceduralSliceInterface.BeforeSlice`
  (params (SlicePlane :type "StaticMeshComponent Object Reference (by ref)") (MotionSource :type "Name (by ref)") (SwingVelocity :type "Float (single-precision) (by ref)"))
  (`KismetSystemLibrary.K2_SetTimer` null "LoadLevel" (`self.LoadLevelTime`)))

(fn `GetSliceMat`
  (returns (SliceMat :type "StaticMaterial Structure"))
  (return (`self.SliceMat`)))

(fn `LoadLevel`
  (`GameplayStatics.OpenLevel` (`self.LevelName`)))

(fn `UserConstructionScript`
  (`KismetProceduralMeshLibrary.CopyProceduralMeshFromStaticMeshComponent` (`self.Cube`) 0 (`self.ProceduralMesh`) true)
  (`TextRenderComponent.K2_SetText` (`self.TextRender`) (`KismetTextLibrary.Conv_NameToText` (`self.LevelName`))))