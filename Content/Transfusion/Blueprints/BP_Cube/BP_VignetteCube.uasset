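; BP_VignetteCube is a sliceable menu-style cube with a text label that toggles the UseVignette setting on the Transfusion game instance.
; The construction script copies the static cube into a procedural mesh, sets both text renders and caches the mesh transform.
; BeforeSlice flips the setting, then after a delay restores the transform, disables physics and rebuilds the mesh.
; A separate event destroys sliced halves after a delay, and GetSliceMat supplies the slice material.
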(event `/Game/Transfusion/Blueprints/Interfaces/IProceduralSliceInterface.BeforeSlice`
  (params (SlicePlane :type "StaticMeshComponent Object Reference (by ref)") (MotionSource :type "Name (by ref)") (SwingVelocity :type "Float (single-precision) (by ref)"))
  (bind _proceduralmesh (`self.ProceduralMesh`))
  (bind _astransfusion_game_instance (cast `/Game/Transfusion/Blueprints/Globals/Transfusion_GameInstance` (`GameplayStatics.GetGameInstance`)))
  (set `/Game/Transfusion/Blueprints/Globals/Transfusion_GameInstance.useVignette` (not (`/Game/Transfusion/Blueprints/Globals/Transfusion_GameInstance.useVignette` _astransfusion_game_instance)) _astransfusion_game_instance)
  (`KismetSystemLibrary.Delay` 2.0)
  (`SceneComponent.K2_SetWorldTransform` _proceduralmesh (`self.CachedWorldTransform`) false false)
  (`PrimitiveComponent.SetSimulatePhysics` _proceduralmesh false)
  (`KismetProceduralMeshLibrary.CopyProceduralMeshFromStaticMeshComponent` (`self.Cube`) 0 (`self.ProceduralMesh`) true))

(event `DestroyProceduralHalvesWithDelay`
  (params (Half1 :type "PrimitiveComponent Object Reference"))
  (`KismetSystemLibrary.Delay` 2.0)
  (`ActorComponent.K2_DestroyComponent` Half1))

(fn `GetSliceMat`
  (returns (SliceMat :type "StaticMaterial Structure"))
  (return (`self.SliceMat`)))

(fn `UserConstructionScript`
  (bind _text (`self.Text`))
  (`KismetProceduralMeshLibrary.CopyProceduralMeshFromStaticMeshComponent` (`self.Cube`) 0 (`self.ProceduralMesh`) true)
  (`TextRenderComponent.K2_SetText` (`self.TextRender`) _text)
  (`TextRenderComponent.K2_SetText` (`self.TextRenderShadow`) _text)
  (set `self.CachedWorldTransform` (`SceneComponent.K2_GetComponentToWorld` (`self.ProceduralMesh`))))