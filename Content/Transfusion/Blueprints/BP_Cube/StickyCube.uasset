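; StickyCube is a cube actor that sticks to a BP_Sword_Legacy2 sword when the two collide.
; On hit, it sets the physics constraint's first-frame reference to the hit location and constrains its HitBox to the sword mesh, allowing one attachment at a time.
; Tick monitors the linear constraint force, and past a high threshold it prints the force and breaks the constraint, allowing the cube to stick again.
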(event `self.ReceiveActorBeginOverlap`
  (params (OtherActor :type "Actor Object Reference")))

(event `self.ReceiveHit`
  (params (MyComp :type "PrimitiveComponent Object Reference") (Other :type "Actor Object Reference") (OtherComp :type "PrimitiveComponent Object Reference") (bSelfMoved :type Boolean) (HitLocation :type "Vector Structure") (HitNormal :type "Vector Structure") (NormalImpulse :type "Vector Structure") (Hit :type "HitResult Structure (by ref)"))
  (bind _physicsconstraint (`self.PhysicsConstraint`))
  (bind _asbp_sword_legacy_2 (cast `/Game/Transfusion/Blueprints/PlayerInteractibles/BP_Sword/BP_Sword_Legacy2` Other))
  (if (not (`self.isConstrained`))
    (set `self.isConstrained` true)
    (`PhysicsConstraintComponent.SetConstraintReferencePosition` _physicsconstraint "Frame1" HitLocation)
    (`PhysicsConstraintComponent.SetConstrainedComponents` _physicsconstraint (`self.HitBox`) "None" (`/Game/Transfusion/Blueprints/PlayerInteractibles/BP_Sword/BP_Sword_Legacy2.SwordMesh` _asbp_sword_legacy_2) "None")))

(event `self.ReceiveTick`
  (params (DeltaSeconds :type "Float (single-precision)"))
  (bind _physicsconstraint (`self.PhysicsConstraint`))
  (if (`self.isConstrained`)
    (bind _outlinearforce (`PhysicsConstraintComponent.GetConstraintForce` _physicsconstraint))
    (bind _returnvalue (`KismetMathLibrary.VSize` _outlinearforce))
    (if (> _returnvalue 10000000.0)
      (`KismetSystemLibrary.PrintString` (`KismetStringLibrary.Conv_DoubleToString` _returnvalue))
      (set `self.isConstrained` false)
      (`PhysicsConstraintComponent.BreakConstraint` _physicsconstraint))))

(fn `UserConstructionScript`)