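; Combat director that paces enemy attacks on the VR player (or a VR dummy) by choosing one enemy to attack on a looping timer.
; Each cycle multiplies every enemy's grade by how opposed its facing is to the player's, then triggers AIAttack on the top-graded enemy's controller and re-rolls its grade randomly.
; Also tracks AI states and creates optional debug widgets showing each enemy's grade and state.
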(event `self.ReceiveBeginPlay`
  (bind _returnvalue (`GameplayStatics.GetActorOfClass` "/Game/Transfusion/Blueprints/VRPawn_Main.VRPawn_Main_C"))
  (`/Engine/EditorBlueprintResources/StandardMacros.IsValid` _returnvalue
    (:`Is Valid`
      (set `self.PlayerRef` _returnvalue))
    (:`Is Not Valid`
      (bind _returnvalue_2 (`GameplayStatics.GetActorOfClass` "/Game/Transfusion/Blueprints/Legacy/BP_VRDummy/BP_VRDummy.BP_VRDummy_C"))
      (set `self.PlayerRef` _returnvalue_2)))
  (`KismetSystemLibrary.K2_SetTimerDelegate` (delegate `Trigger_Attack`) (`self.ScoreCooldown`) true))

(event `Trigger_Attack`
  (if (not (== (`self.Enemy Alive`) 0))
    (`self.RecalculateScores`)
    (bind (_loc_highestvalue1 _loc_highestgradedai1) (`self.FindHighestGrade`))
    (`BlueprintMapLibrary.Map_Add` (`self.EnemyGrading`) _loc_highestgradedai1 (`KismetMathLibrary.RandomFloatInRange` 1.0 5.0))
    (bind _asenemy_controller (cast `/Game/Transfusion/BehaviorTree/EnemyController` (`AIBlueprintHelperLibrary.GetAIController` _loc_highestgradedai1)))
    (`/Game/Transfusion/BehaviorTree/EnemyController.AI_Attack` _asenemy_controller)
    (`self.UpdateDebugWidgets` _loc_highestgradedai1)))

(event `self.ReceiveTick`
  (params (DeltaSeconds :type "Float (single-precision)")))

(fn `AddDebugWidgets`
  (params (`Enemy Instance` :type "Actor Object Reference (by ref)"))
  (locals (Loc_Widget :type "/Game/Transfusion/Widgets/Debug_EnemyAI_Widget Object Reference"))
  (bind _enemygrading (`self.EnemyGrading`))
  (bind _enemy_instance (`local.Enemy Instance`))
  (bind _value (`BlueprintMapLibrary.Map_Find` _enemygrading (`local.Enemy Instance`)))
  ;[1 1 1] Make Interface
  (bind _asbp_lizard_enemy_base (cast `/Game/Transfusion/Blueprints/BP_Enemy/BP_LizardEnemy_Base` `Enemy Instance`)
    (:`then`
      (if (not (`/Game/Transfusion/Blueprints/BP_Enemy/BP_LizardEnemy_Base.HasWidget` _asbp_lizard_enemy_base))
        (`BlueprintMapLibrary.Map_Add` _enemygrading (`local.Enemy Instance`) (`KismetMathLibrary.RandomFloatInRange` 1.0 5.0) :!label _label)
        ;[1 1 1] Make Interface
        (bind _asslicing_dummy_ai (cast `/Game/Transfusion/Blueprints/BP_Enemy/Slicing_Dummy/Slicing_Dummy_AI` (`local.Enemy Instance`))
          (:`then`
            (bind _returnvalue (`|CreateWidget` "/Game/Transfusion/Widgets/Debug_EnemyAI_Widget.Debug_EnemyAI_Widget_C" null _asslicing_dummy_ai _value))
            (set `local.Loc_Widget` _returnvalue))
          (:`CastFailed`
            (bind _asbp_lizard_enemy_base_2 (cast `/Game/Transfusion/Blueprints/BP_Enemy/BP_LizardEnemy_Base` (`local.Enemy Instance`))
              (:`then`
                (bind _returnvalue_2 (`|CreateWidget` "/Game/Transfusion/Widgets/Debug_EnemyAI_Widget.Debug_EnemyAI_Widget_C" null _asbp_lizard_enemy_base_2 _value))
                (set `local.Loc_Widget` _returnvalue_2))
              (:`CastFailed`
                (bind _asbp_lizard_enemy_test (cast `/Game/Transfusion/Blueprints/BP_Enemy/BP_LizardEnemy_Test` (`local.Enemy Instance`)))
                (bind _returnvalue_3 (`|CreateWidget` "/Game/Transfusion/Widgets/Debug_EnemyAI_Widget.Debug_EnemyAI_Widget_C" null _asbp_lizard_enemy_test _value))
                (set `local.Loc_Widget` _returnvalue_3)))))
        (`BlueprintMapLibrary.Map_Add` (`self.EnemyWidgets`) _enemy_instance (`local.Loc_Widget`))
        (if (`self.Enable Debug Widget`)
          (bind _returnvalue_4 (`AddComponent|NODE_AddWidgetComponent-0` :`self` _enemy_instance))
          (`WidgetComponent.SetWidget` _returnvalue_4 (`local.Loc_Widget`)))
        (bind _asbp_lizard_enemy_base_3 (cast `/Game/Transfusion/Blueprints/BP_Enemy/BP_LizardEnemy_Base` _enemy_instance)
          (:`then`
            (set `/Game/Transfusion/Blueprints/BP_Enemy/BP_LizardEnemy_Base.HasWidget` true _asbp_lizard_enemy_base_3))
          (:`CastFailed`
            (bind _asslicing_dummy_ai_2 (cast `/Game/Transfusion/Blueprints/BP_Enemy/Slicing_Dummy/Slicing_Dummy_AI` _enemy_instance)
              (:`then`
                (set `/Game/Transfusion/Blueprints/BP_Enemy/Slicing_Dummy/Slicing_Dummy_AI.HasWidget` true _asslicing_dummy_ai_2))
              (:`CastFailed`
                (bind _asbp_lizard_enemy_test_2 (cast `/Game/Transfusion/Blueprints/BP_Enemy/BP_LizardEnemy_Test` _enemy_instance))
                (set `/Game/Transfusion/Blueprints/BP_Enemy/BP_LizardEnemy_Test.HasWidget` true _asbp_lizard_enemy_test_2)))))))
    (:`CastFailed`
      (bind _asslicing_dummy_ai_3 (cast `/Game/Transfusion/Blueprints/BP_Enemy/Slicing_Dummy/Slicing_Dummy_AI` `Enemy Instance`)
        (:`then`
          (if (not (`/Game/Transfusion/Blueprints/BP_Enemy/Slicing_Dummy/Slicing_Dummy_AI.HasWidget` _asslicing_dummy_ai_3))
            (goto _label)))
        (:`CastFailed`
          (bind _asbp_lizard_enemy_test_3 (cast `/Game/Transfusion/Blueprints/BP_Enemy/BP_LizardEnemy_Test` `Enemy Instance`))
          (if (not (`/Game/Transfusion/Blueprints/BP_Enemy/BP_LizardEnemy_Test.HasWidget` _asbp_lizard_enemy_test_3))
            (goto _label)))))))

(fn `ClearEnemyREFs`
  (`KismetArrayLibrary.Array_Clear` (`self.EnemyList`))
  (`BlueprintMapLibrary.Map_Clear` (`self.EnemyGrading`))
  (`BlueprintMapLibrary.Map_Clear` (`self.EnemyStates`))
  (`BlueprintMapLibrary.Map_Clear` (`self.EnemyWidgets`)))

(fn `FindHighestGrade`
  (returns (Loc_HighestValue1 :type "Float (double-precision)") (Loc_HighestGradedAI1 :type "Actor Object Reference"))
  (locals (Loc_HighestValue :type "Float (double-precision)") (Loc_HighestGradedAI :type "Actor Object Reference"))
  (bind _keys (`BlueprintMapLibrary.Map_Keys` (`self.EnemyGrading`)))
  (for _array_element _keys
    (bind _value (`BlueprintMapLibrary.Map_Find` (`self.EnemyGrading`) _array_element))
    (if (> _value (`local.Loc_HighestValue`))
      (set `local.Loc_HighestValue` _value)
      (set `local.Loc_HighestGradedAI` _array_element)))
  (return (`local.Loc_HighestValue`) (`local.Loc_HighestGradedAI`)))

(fn `RecalculateScores`
  (`self.ScoreByPosition`))

(fn `ScoreByPosition`
  (bind _enemygrading (`self.EnemyGrading`))
  (if (!= (`KismetArrayLibrary.Array_Length` (`self.EnemyList`)) 0)
    (bind _asvrpawn_main (cast `/Game/Transfusion/Blueprints/VRPawn_Main` (`self.PlayerRef`))
      (:`then`
        (for _array_element (`self.EnemyList`)
          (`BlueprintMapLibrary.Map_Add` (`self.EnemyGrading`) _array_element (* (`BlueprintMapLibrary.Map_Find` (`self.EnemyGrading`) _array_element) (+ (`KismetMathLibrary.NormalizeToRange` (* (`KismetMathLibrary.Dot_VectorVector` (`self.GetActorForwardVector` _array_element) (`KismetMathLibrary.GetForwardVector` (`SceneComponent.K2_GetComponentRotation` (`/Game/Transfusion/Blueprints/VRPawn_Main.Camera` _asvrpawn_main)))) -1.0) -1.0 1.0) 0.5)))
          (bind _asenemy_controller (cast `/Game/Transfusion/BehaviorTree/EnemyController` (`AIBlueprintHelperLibrary.GetAIController` _array_element)))
          (`BlueprintMapLibrary.Map_Add` (`self.EnemyStates`) _array_element (`/Game/Transfusion/BehaviorTree/EnemyController.CurrentState` _asenemy_controller))
          (`self.UpdateDebugWidgets` _array_element)))
      (:`CastFailed`
        (bind _asbp_vrdummy (cast `/Game/Transfusion/Blueprints/Legacy/BP_VRDummy/BP_VRDummy` (`self.PlayerRef`)))
        (for _array_element_2 (`self.EnemyList`)
          (`BlueprintMapLibrary.Map_Add` _enemygrading _array_element_2 (* (`BlueprintMapLibrary.Map_Find` _enemygrading _array_element_2) (+ (`KismetMathLibrary.NormalizeToRange` (* (`KismetMathLibrary.Dot_VectorVector` (`self.GetActorForwardVector` _array_element_2) (`SceneComponent.GetForwardVector` (`/Game/Transfusion/Blueprints/Legacy/BP_VRDummy/BP_VRDummy.StaticMesh` _asbp_vrdummy))) -1.0) -1.0 1.0) 0.5)))
          (bind _asenemy_controller_2 (cast `/Game/Transfusion/BehaviorTree/EnemyController` (`AIBlueprintHelperLibrary.GetAIController` _array_element_2)))
          (`BlueprintMapLibrary.Map_Add` (`self.EnemyStates`) _array_element_2 (`/Game/Transfusion/BehaviorTree/EnemyController.CurrentState` _asenemy_controller_2))
          (`self.UpdateDebugWidgets` _array_element_2))))
    (else
      (`KismetSystemLibrary.PrintString` "Unable to find enemies"))))

(fn `UpdateDebugWidgets`
  (params (EnemyInstance :type "Actor Object Reference"))
  (bind _value (`BlueprintMapLibrary.Map_Find` (`self.EnemyWidgets`) EnemyInstance))
  (set `/Game/Transfusion/Widgets/Debug_EnemyAI_Widget.CombatGrade` (`BlueprintMapLibrary.Map_Find` (`self.EnemyGrading`) EnemyInstance) _value)
  (set `/Game/Transfusion/Widgets/Debug_EnemyAI_Widget.AIState` (`BlueprintMapLibrary.Map_Find` (`self.EnemyStates`) EnemyInstance) _value))

(fn `UserConstructionScript`)