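; Wave manager that spawns AI enemy waves and advances once the combat director's enemies are dead, waiting while the VR player is paused.
; A data table row sets the mode: level waves spawn listed classes at random or specific spawners until the last wave.
; Arcade waves keep coming, ramping enemy counts, then capping by Overdrive state.
; Arcade enemy types are weighted random picks from a spawn-info table, queued before spawning.
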(event `self.ReceiveBeginPlay`
  (`KismetSystemLibrary.Delay` 10.0)
  (`self.Initialize`)
  (`self.Spawn Next Wave`))

(event `Spawn Next Wave`
  (bind _asvrpawn_main (cast `/Game/Transfusion/Blueprints/VRPawn_Main` (`GameplayStatics.GetPlayerPawn` 0))
    (:`then`
      (if (`/Game/Transfusion/Blueprints/VRPawn_Main.isPaused` _asvrpawn_main) :!label _label
        (`KismetSystemLibrary.Delay` 1.0)
        (goto _label)
        (else
          (if (`|EnumEquality` (`self.CurrentMode`) "NewEnumerator0") :!label _label_2
            (`self.SpawnCurrentWave`)
            ;[1 1 1] Check Enemies Remaining
            (bind _alldefeated_ (`self.CheckEnemiesRemaining` :!label _label_3))
            (if _alldefeated_
              ;[1 1 1] Play Wave Complete Sound
              (if (`|EnumEquality` (`self.CurrentMode`) "NewEnumerator0")
                (`KismetSystemLibrary.PrintString` (`KismetStringLibrary.Concat_StrStr` "Wave: " (`KismetStringLibrary.Conv_IntToString` (+ (`self.CurrentWave`) 1)) " Completed"))
                (else
                  (`KismetSystemLibrary.PrintString` (`KismetStringLibrary.Concat_StrStr` "Wave: " (`KismetStringLibrary.Conv_IntToString` (+ (`self.CurrentWaveArcade`) 1)) " Completed"))))
              ;[1 1 1] Final Wave? (Level Mode)
              (`KismetSystemLibrary.Delay` 2.0)
              (if (and (== (`self.CurrentWave`) (`KismetArrayLibrary.Array_LastIndex` (`.waveInfo_3_864812DD42423A889082E68359C8139D` (break `/Game/Transfusion/Blueprints/EnemyManagers/S_WaveInfo` (`self.WaveSettings`))))) (`|EnumEquality` (`self.CurrentMode`) "NewEnumerator0"))
                (`self.Final Wave Finished`)
                (else
                  (`/Game/Transfusion/Blueprints/EnemyManagers/BP_CombatDirector.ClearEnemyREFs` (`self.CombatDirectorREF`))
                  (if (`|EnumEquality` (`self.CurrentMode`) "NewEnumerator0")
                    (`/Engine/EditorBlueprintResources/StandardMacros.IncrementInt` (`self.CurrentWave`)
                      (:`  `
                        _))
                    (else
                      (`/Engine/EditorBlueprintResources/StandardMacros.IncrementInt` (`self.CurrentWaveArcade`)
                        (:`  `
                          _))))
                  (`self.Spawn Next Wave`)))
              (else
                (`KismetSystemLibrary.Delay` 1.0)
                (goto _label_3)))
            (elif (`|EnumEquality` (`self.CurrentMode`) "NewEnumerator1")
              (`self.Spawn Current Wave Arcade`)
              (goto _label_3))))))
    (:`CastFailed`
      (if (`self.DebugMode`)
        (goto _label_2)
        (else
          (`KismetSystemLibrary.PrintString` "No Player or Debug Dummy"))))))

(event `Final Wave Finished`
  (`KismetSystemLibrary.PrintString` "Finished Level"))

(fn `CalculateEnemyType`
  (params (Value :type Integer))
  (returns (ID :type Integer))
  (locals (Value_Loc :type Integer) (RangeStart :type Integer) (RangeEnd :type Integer))
  (set `local.Value_Loc` Value)
  (set `local.RangeStart` 0)
  (set `local.RangeEnd` (- (`|GetArrayItem` (`self.EnemyWeights`)) 1))
  (for (_ _array_index) (`self.EnemyWeights`)
    (if (not (== _array_index 0))
      (set `local.RangeStart` (+ (`local.RangeEnd`) 1))
      (if (`KismetArrayLibrary.Array_IsValidIndex` (`self.EnemyWeights`) (+ _array_index 1))
        (set `local.RangeEnd` (+ (`local.RangeEnd`) (`|GetArrayItem` (`self.EnemyWeights`) (+ _array_index 1))))
        (else
          (set `local.RangeEnd` (- (`self.TotalSpawnWeight`) 1)))))
    ;[1 1 1] Is the value within the range
    (if (and (>= (`local.Value_Loc`) (`local.RangeStart`)) (<= (`local.Value_Loc`) (`local.RangeEnd`)))
      (return _array_index)))
  (return 0))

(fn `CalculateTotalSpawnWeight`
  (set `self.TotalSpawnWeight` 0)
  (for (_array_element _array_index) (`self.EnemyStartRounds`)
    (if (<= _array_element (`self.CurrentEnemySpawnArcade`))
      (set `self.TotalSpawnWeight` (+ (`self.TotalSpawnWeight`) (`|GetArrayItem` (`self.EnemyWeights`) _array_index))))))

(fn `CheckEnemiesRemaining`
  (returns (`AllDefeated?` :type Boolean))
  (if (`self.HasWaveSpawned`)
    (for _array_element (`/Game/Transfusion/Blueprints/EnemyManagers/BP_CombatDirector.EnemyList` (`self.CombatDirectorREF`))
      (`/Engine/EditorBlueprintResources/StandardMacros.IsValid` _array_element
        (:`Is Valid`
          (if (`KismetSystemLibrary.DoesImplementInterface` _array_element "/Game/Transfusion/Blueprints/Interfaces/IEnemyInterface.IEnemyInterface_C")
            (bind _is_alive (message `/Game/Transfusion/Blueprints/Interfaces/IEnemyInterface.Is Alive` _array_element))
            (if _is_alive
              (return false))))))
    (return true)
    (else
      (return false))))

(fn `CheckMode`
  (bind _output (`|GetArrayItem` (`.ClassAmount_7_75D1C9C344C5568AFFB9759E0A3F0586` (break `/Game/Transfusion/Blueprints/EnemyManagers/S_EnemyInfo` (`|GetArrayItem` (`.waveInfo_3_864812DD42423A889082E68359C8139D` (break `/Game/Transfusion/Blueprints/EnemyManagers/S_WaveInfo` (`self.WaveSettings`))) (`self.CurrentWave`))))))
  (if (> _output 0)
    (set `self.CurrentMode` "NewEnumerator0")
    (elif (== _output 0)
      (set `self.CurrentMode` "NewEnumerator2")
      (elif (< _output 0)
        (set `self.CurrentMode` "NewEnumerator1")
        (`KismetSystemLibrary.PrintString` "ARCADE MODE")
        (else
          (`KismetSystemLibrary.PrintString` "No Mode is Set"))))))

(fn `GetRandomSpawnPoint`
  (returns (SpawnLocation :type "Vector Structure"))
  (bind _spawn_volume (`/Game/Transfusion/Blueprints/EnemyManagers/BP_EnemySpawner.Spawn Volume` (`KismetArrayLibrary.Array_RandomFromStream` (`self.SpawnersREF`) (`self.RandomStream`))))
  (return (`KismetMathLibrary.RandomPointInBoundingBox` (`SceneComponent.K2_GetComponentLocation` _spawn_volume) (`BoxComponent.GetScaledBoxExtent` _spawn_volume))))

(fn `GetSpecificSpawnPoint`
  (params (SpawnerIndex :type Integer))
  (returns (SpawnLocation :type "Vector Structure"))
  (bind _spawn_volume (`/Game/Transfusion/Blueprints/EnemyManagers/BP_EnemySpawner.Spawn Volume` (`|GetArrayItem` (`self.SpawnersREF`) SpawnerIndex)))
  (return (`KismetMathLibrary.RandomPointInBoundingBox` (`SceneComponent.K2_GetComponentLocation` _spawn_volume) (`BoxComponent.GetScaledBoxExtent` _spawn_volume))))

(fn `Initialize`
  ;[1 1 1] Data Table
  (bind _returnvalue (`|GetDataTableRow` "/Game/Transfusion/Blueprints/EnemyManagers/DT_WaveInfo.DT_WaveInfo" (`self.ArcadeRowName`))
    (:`then`
      (set `self.WaveSettings` _returnvalue)
      (bind _returnvalue_2 (`GameplayStatics.GetActorOfClass` "/Game/Transfusion/Blueprints/EnemyManagers/BP_CombatDirector.BP_CombatDirector_C"))
      (set `self.CombatDirectorRef` _returnvalue_2)
      ;[1 1 1] Spawn Points
      (bind _outactors (`GameplayStatics.GetAllActorsOfClass` "/Game/Transfusion/Blueprints/EnemyManagers/BP_EnemySpawner.BP_EnemySpawner_C"))
      (set `self.SpawnersREF` _outactors)
      ;[1 1 1] Set Seed
      (`KismetMathLibrary.SetRandomStreamSeed` (`self.RandomStream`) (`self.Seed`))
      ;[1 1 1] Check Mode and Set Mode Enum
      (`self.CheckMode`)
      ;[1 1 1] Set Enemy Variables from Enemy DT
      (`self.SetEnemyVars`)
      ;[1 1 1] Handle Initial Conditions and Countdown
      (`KismetSystemLibrary.PrintString` "Countdown")
      (bind _returnvalue_3 (`GameplayStatics.GetActorOfClass` "/Game/Transfusion/Blueprints/Legacy/BP_VRDummy/BP_VRDummy.BP_VRDummy_C"))
      (`/Engine/EditorBlueprintResources/StandardMacros.IsValid` _returnvalue_3
        (:`Is Valid`
          (set `self.DebugMode` true))))))

(fn `PrintEnemyQueue`
  (locals (Queue :type String))
  (set `local.Queue` "")
  (for _array_element (`self.EnemyQueue`)
    (set `local.Queue` (`KismetStringLibrary.Concat_StrStr` (`local.Queue`) (`KismetStringLibrary.Conv_IntToString` _array_element)))
    (set `local.Queue` (`KismetStringLibrary.Concat_StrStr` (`local.Queue`) ", ")))
  (`KismetSystemLibrary.PrintString` (`local.Queue`)))

(fn `SetEnemyVars`
  (if (`|EnumEquality` (`self.CurrentMode`) "NewEnumerator1")
    (bind _outrownames (`DataTableFunctionLibrary.GetDataTableRowNames` "/Game/Transfusion/Blueprints/EnemyManagers/DT_EnemySpawnInfo.DT_EnemySpawnInfo"))
    (for _array_element _outrownames
      (bind _returnvalue (`|GetDataTableRow` "/Game/Transfusion/Blueprints/EnemyManagers/DT_EnemySpawnInfo.DT_EnemySpawnInfo" _array_element)
        (:`then`
          (bind (_id _enemyclass _startround _requiredamount _spawnweights) (break `/Game/Transfusion/Blueprints/EnemyManagers/S_SpawnInfo` _returnvalue))
          (`KismetArrayLibrary.Array_Add` (`self.EnemyTypes`) _enemyclass)
          (`KismetArrayLibrary.Array_Add` (`self.EnemyStartRounds`) _startround)
          (`KismetArrayLibrary.Array_Add` (`self.EnemyWeights`) _spawnweights))))))

(fn `Spawn Current Wave Arcade`
  (set `self.HasWaveSpawned` false)
  (if (< (`self.CurrentWaveArcade`) 7)
    ;[1 1 1] Initial Six Rounds
    (switch `int` (`self.CurrentWaveArcade`)
      (:`0`
        _)
      (:`1`
        (set `self.CurrentEnemySpawnArcade` (+ (`self.CurrentEnemySpawnArcade`) (`self.EnemyIncrement`)) :!label _label))
      (:`2`
        (goto _label))
      (:`3`
        _)
      (:`4`
        (goto _label))
      (:`5`
        _)
      (:`6`
        (set `self.CurrentEnemySpawnArcade` (+ (`self.CurrentEnemySpawnArcade`) (`self.OverdriveEnemyIncrement`)))))
    (else
      ;[1 1 1] Determine Overdrive Increment
      (bind _asvrgame_mode (cast `/Game/Transfusion/Blueprints/Globals/VRGameMode` (`GameplayStatics.GetGameMode`)))
      (if (`/Game/Transfusion/Blueprints/Globals/VRGameMode.InOverdrive` _asvrgame_mode)
        (set `self.CurrentEnemySpawnArcade` (`self.OverdriveMaxEnemySpawn`))
        (else
          (set `self.CurrentEnemySpawnArcade` (`self.DefaultMaxEnemySpawn`))))))
  (`self.CalculateTotalSpawnWeight`)
  (`KismetArrayLibrary.Array_Clear` (`self.EnemyQueue`))
  ;[1 1 1] Calculate Enemy Queue (Add ID to array)
  (for _ (range (`self.CurrentEnemySpawnArcade`))
    (`KismetArrayLibrary.Array_Add` (`self.EnemyQueue`) (`self.CalculateEnemyType` (`KismetMathLibrary.RandomIntegerInRange` 0 (- (`self.TotalSpawnWeight`) 1)))))
  (`self.PrintEnemyQueue`)
  ;[1 1 1] Spawn Enemies in Queue
  (for _array_element (`self.EnemyQueue`)
    (bind _output (`|GetArrayItem` (`self.EnemyTypes`) _array_element))
    (`AIBlueprintHelperLibrary.SpawnAIFromClass` _output "/Game/Transfusion/BehaviorTree/Enemy_BT.Enemy_BT" (`self.GetRandomSpawnPoint`) (struct) true null :!pinned true) ; Spawn at Random Spawner
    (`KismetSystemLibrary.PrintString` (`KismetStringLibrary.Concat_StrStr` "Spawned: " (`KismetSystemLibrary.GetClassDisplayName` _output))))
  (set `self.HasWaveSpawned` true))

(fn `SpawnCurrentWave`
  (bind (_enemyclasses _classamount _spawnerid) (break `/Game/Transfusion/Blueprints/EnemyManagers/S_EnemyInfo` (`|GetArrayItem` (`.waveInfo_3_864812DD42423A889082E68359C8139D` (break `/Game/Transfusion/Blueprints/EnemyManagers/S_WaveInfo` (`self.WaveSettings`))) (`self.CurrentWave`))))
  (set `self.HasWaveSpawned` false)
  (for (_array_element _array_index) _enemyclasses
    (for _ (range (`|GetArrayItem` _classamount _array_index))
      (bind _output (`|GetArrayItem` _spawnerid _array_index))
      (if (== _output -1)
        (`AIBlueprintHelperLibrary.SpawnAIFromClass` _array_element "/Game/Transfusion/BehaviorTree/Enemy_BT.Enemy_BT" (`self.GetRandomSpawnPoint`) (struct) true null :!pinned true) ; Spawn at Random Spawner
        (elif (`KismetArrayLibrary.Array_IsValidIndex` (`self.SpawnersREF`) _output)
          (`AIBlueprintHelperLibrary.SpawnAIFromClass` _array_element "/Game/Transfusion/BehaviorTree/Enemy_BT.Enemy_BT" (`self.GetSpecificSpawnPoint` _output) (struct) true null :!pinned true) ; Spawn at Specific Spawner
        ))))
  (set `self.HasWaveSpawned` true))

(fn `SpawnCurrentWaveLegacy`
  (bind (_enemyclasses _classamount) (break `/Game/Transfusion/Blueprints/EnemyManagers/S_EnemyInfo` (`|GetArrayItem` (`.waveInfo_3_864812DD42423A889082E68359C8139D` (break `/Game/Transfusion/Blueprints/EnemyManagers/S_WaveInfo` (`self.WaveSettings`))) (`self.CurrentWave`))))
  (for (_array_element _array_index) _enemyclasses
    (for _ (range (`|GetArrayItem` _classamount _array_index))
      (`AIBlueprintHelperLibrary.SpawnAIFromClass` _array_element "/Game/Transfusion/BehaviorTree/Enemy_BT.Enemy_BT" (`self.GetRandomSpawnPoint`) (struct) true null))))

(fn `UserConstructionScript`)