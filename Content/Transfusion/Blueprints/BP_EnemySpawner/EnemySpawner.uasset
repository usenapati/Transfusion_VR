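; Enemy spawner that spawns growing waves of AI enemies at random points in its SpawnVolume whenever the CombatDirector fires RespawnEnemy.
; Each spawned Slicing_Dummy_AI or BP_LizardEnemy_Base gets DamageIncrement added to its base damage.
; After each wave the count grows, with VRGameMode's Overdrive state selecting the increment and cap.
; Once the count reaches the cap it is clamped and DamageIncrement doubles instead.
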(event `self.ReceiveBeginPlay`
  (bind _returnvalue (`GameplayStatics.GetActorOfClass` "/Game/Transfusion/BehaviorTree/CombatDirector.CombatDirector_C"))
  (bind _output_get (set `self.CombatDirectorRef` _returnvalue))
  (add `/Game/Transfusion/BehaviorTree/CombatDirector.RespawnEnemy` _output_get (delegate `SpawnEnemy`)))

(event `SpawnEnemy`
  (bind _spawn_volume (`self.Spawn Volume`))
  (set `self.CanSpawn` true)
  (for _ (range (`self.EnemySpawned`))
    (set `self.CanSpawn` false)
    ;[1 1 1] UPDATE ME
    (bind _returnvalue (`AIBlueprintHelperLibrary.SpawnAIFromClass` (`self.Enemy Class`) "/Game/Transfusion/BehaviorTree/Enemy_BT.Enemy_BT" (`KismetMathLibrary.RandomPointInBoundingBox` (`SceneComponent.K2_GetComponentLocation` _spawn_volume) (`BoxComponent.GetScaledBoxExtent` _spawn_volume)) (struct) true null))
    (bind _asslicing_dummy_ai (cast `/Game/Transfusion/Blueprints/BP_Enemy/Slicing_Dummy/Slicing_Dummy_AI` _returnvalue)
      (:`then`
        (set `/Game/Transfusion/Blueprints/BP_Enemy/Slicing_Dummy/Slicing_Dummy_AI.BaseDamage` (+ (`/Game/Transfusion/Blueprints/BP_Enemy/Slicing_Dummy/Slicing_Dummy_AI.BaseDamage` _asslicing_dummy_ai) (`self.Damage Increment`)) _asslicing_dummy_ai)
        (`KismetSystemLibrary.Delay` (`self.Spawn Delay`))
        (set `self.CanSpawn` true))
      (:`CastFailed`
        (bind _asbp_lizard_enemy_base (cast `/Game/Transfusion/Blueprints/BP_Enemy/BP_LizardEnemy_Base` _returnvalue))
        (set `/Game/Transfusion/Blueprints/BP_Enemy/BP_LizardEnemy_Base.BaseDamage` (+ (`/Game/Transfusion/Blueprints/BP_Enemy/BP_LizardEnemy_Base.BaseDamage` _asbp_lizard_enemy_base) (`self.Damage Increment`)) _asbp_lizard_enemy_base)
        (`KismetSystemLibrary.Delay` (`self.Spawn Delay`))
        (set `self.CanSpawn` true))))
  (if (>= (`self.EnemySpawned`) (`self.CurrentMaximumEnemySpawn`))
    (set `self.EnemySpawned` (`self.CurrentMaximumEnemySpawn`))
    (set `self.Damage Increment` (+ (`self.Damage Increment`) (`self.Damage Increment`)))
    (else
      (bind _asvrgame_mode (cast `/Game/Transfusion/Blueprints/VRGameMode` (`GameplayStatics.GetGameMode`)))
      (if (`/Game/Transfusion/Blueprints/VRGameMode.InOverdrive` _asvrgame_mode)
        (set `self.EnemySpawned` (+ (`self.EnemySpawned`) (`self.OverdriveEnemyIncrement`)))
        (set `self.CurrentMaximumEnemySpawn` (`self.OverdriveMaxEnemySpawn`))
        (else
          (set `self.EnemySpawned` (+ (`self.EnemySpawned`) (`self.EnemyIncrement`)))
          (set `self.CurrentMaximumEnemySpawn` (`self.DefaultMaximumEnemySpawn`)))))))

(fn `UserConstructionScript`)