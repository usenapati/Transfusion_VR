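; VR game mode that tracks the player's combo and drives the crowd and music audio from it.
; BeginPlay near-mutes the pawn's overdrive music and caches the CombatDirector and Music_BA actors.
; AddCombo restarts a reset timer, updates crowd volume and switches to the overdrive loop at a threshold; ResetCombo restores the arena loop.
; Enemy respawn and repeating score-timer logic are left disconnected.
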(event `self.ReceiveBeginPlay`
  (bind _asvrpawn (cast `/Game/Transfusion/Blueprints/VRPawn` (`GameplayStatics.GetPlayerPawn` 0)))
  (`AudioComponent.AdjustVolume` (`/Game/Transfusion/Blueprints/VRPawn.BackgroundMusicOverdrive` _asvrpawn) 0.0 0.001 "Linear")
  (bind _returnvalue (`GameplayStatics.GetActorOfClass` "/Game/Transfusion/BehaviorTree/CombatDirector.CombatDirector_C"))
  (set `self.CombatDirector_REF` _returnvalue)
  (bind _returnvalue_2 (`GameplayStatics.GetActorOfClass` "/Game/Transfusion/Audio/Music_BA.Music_BA_C"))
  (set `self.Music BA REF` _returnvalue_2))

(event `DecrementScoreRepeating`
  ;[1 1 1] Every so often, reduce the crowd score by a set amount
  (`self.AddCombo` 1))

(event `self.ReceiveTick`
  (params (DeltaSeconds :type "Float (single-precision)")))

(event `CheckEnemyLeft`)

(fn `AddCombo`
  (params (Amount :type Integer))
  (`KismetSystemLibrary.K2_ClearTimer` null "ResetCombo")
  (bind _output_get (set `self.Combo` (+ (`self.Combo`) Amount)))
  (`KismetSystemLibrary.K2_SetTimer` null "ResetCombo" (`self.ComboResetTime`))
  (`/Game/Transfusion/Audio/Music_BA.ChangeCrowdVolume` (`self.Music BA REF`) _output_get)
  (if (>= (`self.Combo`) (`self.OverdriveModeThreshold`))
    (`/Game/Transfusion/Audio/Music_BA.SwapToOverdriveLoop` (`self.Music BA REF`))))

(fn `ResetCombo`
  (bind _music_ba_ref (`self.Music BA REF`))
  (bind _output_get (set `self.Combo` 0))
  (cast `/Game/Transfusion/Blueprints/VRPawn` (`GameplayStatics.GetPlayerPawn` 0))
  (`/Game/Transfusion/Audio/Music_BA.ChangeCrowdVolume` _music_ba_ref _output_get)
  (`/Game/Transfusion/Audio/Music_BA.SwapToArenaLoop` _music_ba_ref))

(fn `UserConstructionScript`)