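; BP_MagicGem is a grabbable powerup gem that can be dropped into a socket.
; On BeginPlay it sets its mesh from the GemModels map by MagicType.
; Mesh overlaps with actors implementing I_SocketInterface store the socket and set InSocket, which any end overlap clears.
; Dropping the gem while InSocket is set messages the stored socket to attach it, leaving attachment logic to the socket.
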(event `self.ReceiveBeginPlay`
  (`StaticMeshComponent.SetStaticMesh` (`self.GemModel`) (`BlueprintMapLibrary.Map_Find` (`self.GemModels`) (`self.MagicType`))))

(event `self.GrabComponent.OnDropped`
  (if (`self.inSocket`)
    (message `/Game/Transfusion/Blueprints/Interfaces/I_SocketInterface.AttachGemToSocket` (`self.SocketRef`) self)))

(event `self.GemModel.OnComponentBeginOverlap`
  (params (OverlappedComponent :type "PrimitiveComponent Object Reference") (OtherActor :type "Actor Object Reference") (OtherComp :type "PrimitiveComponent Object Reference") (OtherBodyIndex :type Integer) (bFromSweep :type Boolean) (SweepResult :type "HitResult Structure (by ref)"))
  (if (`KismetSystemLibrary.DoesImplementInterface` OtherActor "/Game/Transfusion/Blueprints/Interfaces/I_SocketInterface.I_SocketInterface_C")
    (set `self.SocketRef` OtherActor)
    (set `self.inSocket` true)))

(event `self.GemModel.OnComponentEndOverlap`
  (params (OverlappedComponent :type "PrimitiveComponent Object Reference") (OtherActor :type "Actor Object Reference") (OtherComp :type "PrimitiveComponent Object Reference") (OtherBodyIndex :type Integer))
  (if (`self.inSocket`)
    (set `self.inSocket` false)))

(fn `BeginGemSocketOverlap`
  (params (ObjectRef :type "Actor Object Reference")))

(fn `EndGemSocketOverlap`)

(fn `UserConstructionScript`)