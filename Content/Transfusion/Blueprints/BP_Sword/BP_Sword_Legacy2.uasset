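; VR sword actor that the player grabs with either hand to slash, stab or throw at enemies.
; Per-hand physics handles drive the mesh toward the motion controller while the hand mesh snaps to the hilt.
; Slash and stab overlap planes check tip travel and velocity, then send body or joint hits or slice procedural meshes.
; Fast releases spin the sword with a resized slash plane; socketed gem powerups persist through the GameInstance.
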(event `self.ReceiveBeginPlay`
  (bind _returnvalue (`GameplayStatics.GetCurrentLevelName` true))
  (if (`KismetStringLibrary.NotEqual_StrStr` _returnvalue "TrainingRoom")
    (bind _astransfusion_game_instance (cast `/Game/Transfusion/Blueprints/Transfusion_GameInstance` (`GameplayStatics.GetGameInstance`)))
    (bind _swordpowerup (`/Game/Transfusion/Blueprints/Transfusion_GameInstance.SwordPowerup` _astransfusion_game_instance))
    (if (`|EnumInequality` _swordpowerup "NewEnumerator6")
      (bind _returnvalue_2 (`|SpawnActorFromClass` "/Game/Transfusion/Blueprints/Powerups/BP_MagicGem.BP_MagicGem_C" (`KismetMathLibrary.MakeTransform` (0.0 0.0 0.0)) "Undefined" "OverrideRootScale" null null))
      (`/Game/Transfusion/Blueprints/Powerups/BP_MagicGem.SetMagicType` _returnvalue_2 _swordpowerup)
      (`self.AttachGemToSocket` _returnvalue_2 _swordpowerup)
      (`PrimitiveComponent.SetCollisionEnabled` (`/Game/Transfusion/Blueprints/Powerups/BP_MagicGem.GemModel` _returnvalue_2) "NoCollision"))))

(event `self.GrabComponent.OnGrabbed`
  ;[1 1 1] Handle Grabbing and Dropping Sword
  (`self.GrabSword`))

(event `self.GrabComponent.OnDropped`
  ;[1 1 1] Handle Grabbing and Dropping Sword
  (`self.ReleaseSword`))

(event `self.ReceiveTick`
  (params (DeltaSeconds :type "Float (single-precision)"))
  ;[1 1 1] Tick
  (if (`/Game/VRTemplate/Blueprints/GrabComponent.bIsHeld` (`self.GrabComponent`))
    (`self.UpdatePhysicsHandle`)
    (`self.IsValidSwing`)))

(event `self.SlashPlane.OnComponentBeginOverlap`
  (params (OverlappedComponent :type "PrimitiveComponent Object Reference") (OtherActor :type "Actor Object Reference") (OtherComp :type "PrimitiveComponent Object Reference") (OtherBodyIndex :type Integer) (bFromSweep :type Boolean) (SweepResult :type "HitResult Structure (by ref)"))
  (bind _componenttags (`ActorComponent.ComponentTags` OtherComp))
  ;[1 1 1] Handle Slashing
  (bind (_isvalidslashtarget _slashtype) (`self.DecideSlashType` OtherActor _componenttags))
  (if _isvalidslashtarget
    (`/Engine/EditorBlueprintResources/StandardMacros.DoOnce` false :!label _label
      (:`Completed`
        (`self.DoSlash` _slashtype OtherActor OtherComp _componenttags SweepResult)))))

(event `self.SlashPlane.OnComponentEndOverlap`
  (params (OverlappedComponent :type "PrimitiveComponent Object Reference") (OtherActor :type "Actor Object Reference") (OtherComp :type "PrimitiveComponent Object Reference") (OtherBodyIndex :type Integer))
  ;[1 1 1] Handle Slashing
  (goto _label :!via `Reset`))

(event `self.StabPlane.OnComponentBeginOverlap`
  (params (OverlappedComponent :type "PrimitiveComponent Object Reference") (OtherActor :type "Actor Object Reference") (OtherComp :type "PrimitiveComponent Object Reference") (OtherBodyIndex :type Integer) (bFromSweep :type Boolean) (SweepResult :type "HitResult Structure (by ref)"))
  (bind _componenttags (`ActorComponent.ComponentTags` OtherComp))
  (bind _returnvalue (`KismetArrayLibrary.Array_Contains` _componenttags "Joint"))
  (bind _returnvalue_2 (`KismetArrayLibrary.Array_Contains` _componenttags "Body"))
  ;[1 1 1] Handle Stabbing
  (if (and (`KismetSystemLibrary.DoesImplementInterface` OtherActor "/Game/Transfusion/Blueprints/Interfaces/IEnemyInterface.IEnemyInterface_C") (`self.CanStab`) (or _returnvalue _returnvalue_2))
    (bind (_isvalidstab _swordstabdistance _swordvelocity) (`self.IsValidStab`))
    (if _isvalidstab
      (set `self.CanStab` false)
      (if _returnvalue
        (message `/Game/Transfusion/Blueprints/Interfaces/IEnemyInterface.Hit Joint` OtherActor 30 _swordstabdistance _swordvelocity _componenttags true SweepResult)
        (`KismetSystemLibrary.PrintString` "Damaged Enemy: STAB JOINT")
        (`KismetSystemLibrary.K2_SetTimer` null "StabTimer" 1.0 :!label _label_2)
        (elif _returnvalue_2
          (message `/Game/Transfusion/Blueprints/Interfaces/IEnemyInterface.Hit Body` OtherActor 20 _swordstabdistance _swordvelocity SweepResult)
          (`KismetSystemLibrary.PrintString` "Damaged Enemy: STAB BODY")
          (goto _label_2))))))

(event `self.StabPlane.OnComponentEndOverlap`
  (params (OverlappedComponent :type "PrimitiveComponent Object Reference") (OtherActor :type "Actor Object Reference") (OtherComp :type "PrimitiveComponent Object Reference") (OtherBodyIndex :type Integer))
  ;[1 1 1] Handle Stabbing
)

(event `self.SwordMesh.OnComponentHit`
  (params (HitComponent :type "PrimitiveComponent Object Reference") (OtherActor :type "Actor Object Reference") (OtherComp :type "PrimitiveComponent Object Reference") (NormalImpulse :type "Vector Structure") (Hit :type "HitResult Structure (by ref)"))
  (if (`self.isAirborn`)
    (`self.ToggleAirborn` false)))

(event `self.AttachGemToSocket`
  (params (Gem :type "Actor Object Reference") (Powerup :type "/Game/Transfusion/Blueprints/Powerups/Enum_Powerups Enum" :default "NewEnumerator0"))
  (if (not (`self.gemInSocket`))
    (`self.K2_AttachToComponent` Gem (`self.SwordMesh`) "GemSocket" "SnapToTarget" "SnapToTarget" "KeepWorld" true)
    (bind _astransfusion_game_instance (cast `/Game/Transfusion/Blueprints/Transfusion_GameInstance` (`GameplayStatics.GetGameInstance`)))
    (set `/Game/Transfusion/Blueprints/Transfusion_GameInstance.SwordPowerup` Powerup _astransfusion_game_instance)
    (set `self.gemInSocket` true)))

(event `self.RemoveGemFromSocket`
  (if (`self.gemInSocket`)
    (bind _astransfusion_game_instance (cast `/Game/Transfusion/Blueprints/Transfusion_GameInstance` (`GameplayStatics.GetGameInstance`)))
    (set `/Game/Transfusion/Blueprints/Transfusion_GameInstance.SwordPowerup` "NewEnumerator6" _astransfusion_game_instance)
    (set `self.gemInSocket` false)))

(fn `DecideSlashType`
  (params (OtherActor :type "Object Object Reference") (`Component Tags` :type "Array of Name (by ref)"))
  (returns (IsValidSlashTarget :type Boolean) (SlashType :type "/Game/Transfusion/Blueprints/BP_Sword/SlashType Enum"))
  (locals (returnSlashType :type "/Game/Transfusion/Blueprints/BP_Sword/SlashType Enum") (returnValidSlashTarget :type Boolean))
  ;[1 1 1] ProceduralSlice path
  (if (`KismetArrayLibrary.Array_Contains` `Component Tags` "Sliceable")
    (set `local.returnSlashType` "NewEnumerator2")
    ;[1 1 1] Valid Slash path
    (if (`self.CanSlash`) :!label _label
      (set `local.returnValidSlashTarget` true))
    (else
      ;[1 1 1] Joint Slash path
      (if (`KismetArrayLibrary.Array_Contains` `Component Tags` "Joint")
        (set `local.returnSlashType` "NewEnumerator1")
        (goto _label)
        (else
          ;[1 1 1] Body Slash path
          (if (`KismetArrayLibrary.Array_Contains` `Component Tags` "Body")
            (set `local.returnSlashType` "NewEnumerator0")
            (goto _label)
            (else
              _))))))
  (return (`local.returnValidSlashTarget`) (`local.returnSlashType`)))

(fn `DoSlash`
  (params (SlashType :type "/Game/Transfusion/Blueprints/BP_Sword/SlashType Enum" :default "NewEnumerator0") (`Other Actor` :type "Actor Object Reference") (OtherComponent :type "PrimitiveComponent Object Reference") (`Component Tags` :type "Array of Name") (Hit :type "HitResult Structure"))
  (locals (SwordSwingDistance :type "Float (double-precision)") (SwordSwingVelocity :type "Float (double-precision)"))
  (bind _swordswingvelocity (`local.SwordSwingVelocity`))
  (bind (_isvalidswing _swordswingdistance _swordvelocity) (`self.IsValidSwing`))
  (if _isvalidswing
    (set `local.SwordSwingDistance` _swordswingdistance)
    (set `local.SwordSwingVelocity` _swordvelocity)
    (set `self.CanSlash` false)
    (switch `/Game/Transfusion/Blueprints/BP_Sword/SlashType` SlashType
      (:`NewEnumerator0`
        (message `/Game/Transfusion/Blueprints/Interfaces/IEnemyInterface.Hit Body` (`local.Other Actor`) 20 (`local.SwordSwingDistance`) (`local.SwordSwingVelocity`) Hit)
        (`KismetSystemLibrary.PrintString` "Damaged Enemy:  SLASH BODY"))
      (:`NewEnumerator1`
        (message `/Game/Transfusion/Blueprints/Interfaces/IEnemyInterface.Hit Joint` (`local.Other Actor`) 30 (`local.SwordSwingDistance`) (`local.SwordSwingVelocity`) (`local.Component Tags`) false Hit)
        (`KismetSystemLibrary.PrintString` "Damaged Enemy:  SLASH JOINT"))
      (:`NewEnumerator2`
        (message `/Game/Transfusion/Blueprints/Interfaces/IProceduralSliceInterface.BeforeSlice` (`local.Other Actor`) (`self.SlashPlane`) (`MotionControllerComponent.MotionSource` (`/Game/VRTemplate/Blueprints/GrabComponent.MotionControllerRef` (`self.GrabComponent`))) _swordswingvelocity)
        (`self.SliceProceduralMesh` _swordswingvelocity (`local.OtherComponent`))))
    ;[1 1 1] Testing this - no timer to reset
    (`KismetSystemLibrary.K2_SetTimer` null "SliceTimer")
    (set `self.CanSlash` true)))

(fn `GiantSwordDisable`
  (bind _slashplane (`self.SlashPlane`))
  ;[1 1 1] Disable
  (`SceneComponent.SetRelativeScale3D` _slashplane (`self.NormalSwordScale`))
  (`SceneComponent.K2_SetRelativeLocation` _slashplane (`self.NormalSwordLocation`) false false)
  ;;[1 1 1] Change Interpolation Speed
  (bind _asvrpawn_main (cast `/Game/Transfusion/Blueprints/VRPawn_Main` (`ActorComponent.GetOwner` (`/Game/VRTemplate/Blueprints/GrabComponent.MotionControllerRef` (`self.GrabComponent`)))))
  (`PhysicsHandleComponent.SetInterpolationSpeed` (`/Game/Transfusion/Blueprints/VRPawn_Main.PhysicsHandleLeft` _asvrpawn_main) (`self.Normal Interpolation Speed`))
  (`KismetSystemLibrary.PrintString` "Disabled Giant Sword"))

(fn `GiantSwordEnable`
  (locals (GiantSword :type Boolean))
  (bind _slashplane (`self.SlashPlane`))
  ;[1 1 1] Enable
  (`SceneComponent.SetRelativeScale3D` _slashplane (`self.GiantSwordScale`))
  (`SceneComponent.K2_SetRelativeLocation` _slashplane (`self.GiantSwordLocation`) false false)
  ;;[1 1 1] Change Interpolation Speed
  (bind _asvrpawn_main (cast `/Game/Transfusion/Blueprints/VRPawn_Main` (`ActorComponent.GetOwner` (`/Game/VRTemplate/Blueprints/GrabComponent.MotionControllerRef` (`self.GrabComponent`)))))
  (`PhysicsHandleComponent.SetInterpolationSpeed` (`/Game/Transfusion/Blueprints/VRPawn_Main.PhysicsHandleLeft` _asvrpawn_main) (`self.Slow Interpolation Speed`))
  (`KismetSystemLibrary.PrintString` "Enabled Giant Sword"))

(fn `GrabSword`
  (bind _swordmesh (`self.SwordMesh`))
  (bind _returnvalue (`SceneComponent.GetSocketLocation` _swordmesh "GrabHandle"))
  (bind _returnvalue_2 (`SceneComponent.K2_GetComponentRotation` _swordmesh))
  (bind _motioncontrollerref (`/Game/VRTemplate/Blueprints/GrabComponent.MotionControllerRef` (`self.GrabComponent`)))
  (bind _motioncontrollerref_2 (`/Game/VRTemplate/Blueprints/GrabComponent.MotionControllerRef` (`self.GrabComponent`)))
  (if (`KismetSystemLibrary.IsValid` (`self.HandCompRef`))
    (`self.ReleaseSword`))
  (`PrimitiveComponent.SetEnableGravity` (`self.SwordMesh`) false)
  (bind _asvrpawn_main (cast `/Game/Transfusion/Blueprints/VRPawn_Main` (`ActorComponent.GetOwner` _motioncontrollerref)))
  (if (== (`MotionControllerComponent.MotionSource` _motioncontrollerref) "LEFT")
    ;[1 1 1] Left Hand Logic
    (`PhysicsHandleComponent.GrabComponentAtLocationWithRotation` (`/Game/Transfusion/Blueprints/VRPawn_Main.PhysicsHandleLeft` _asvrpawn_main) (`self.SwordMesh`) "None" _returnvalue _returnvalue_2)
    (set `self.HandParentRef` _motioncontrollerref_2)
    (bind _output_get (set `self.HandCompRef` (`/Game/Transfusion/Blueprints/VRPawn_Main.HandLeft` _asvrpawn_main)))
    (set `self.HandTransformRef` (`SceneComponent.GetRelativeTransform` _output_get))
    (`SceneComponent.K2_AttachToComponent` _output_get (`self.SwordMesh`) "GrabHandleLeft" "SnapToTarget" "SnapToTarget" "SnapToTarget" true)
    (bind _output_get_2 (set `/Game/Transfusion/Blueprints/VRPawn_Main.LastHeldLeft` (`self.SwordMesh`) _asvrpawn_main))
    (if (== _output_get_2 (`/Game/Transfusion/Blueprints/VRPawn_Main.LastHeldRight` _asvrpawn_main))
      (set `/Game/Transfusion/Blueprints/VRPawn_Main.LastHeldRight` null _asvrpawn_main))
    (else
      ;[1 1 1] Right Hand Logic
      (`PhysicsHandleComponent.GrabComponentAtLocationWithRotation` (`/Game/Transfusion/Blueprints/VRPawn_Main.PhysicsHandleRight` _asvrpawn_main) (`self.SwordMesh`) "None" _returnvalue _returnvalue_2)
      (set `self.HandParentRef` _motioncontrollerref_2)
      (bind _output_get_3 (set `self.HandCompRef` (`/Game/Transfusion/Blueprints/VRPawn_Main.HandRight` _asvrpawn_main)))
      (set `self.HandTransformRef` (`SceneComponent.GetRelativeTransform` _output_get_3))
      (`SceneComponent.K2_AttachToComponent` _output_get_3 (`self.SwordMesh`) "GrabHandle" "SnapToTarget" "SnapToTarget" "SnapToTarget" true)
      (bind _output_get_4 (set `/Game/Transfusion/Blueprints/VRPawn_Main.LastHeldRight` (`self.SwordMesh`) _asvrpawn_main))
      (if (== _output_get_4 (`/Game/Transfusion/Blueprints/VRPawn_Main.LastHeldLeft` _asvrpawn_main))
        (set `/Game/Transfusion/Blueprints/VRPawn_Main.LastHeldLeft` null _asvrpawn_main))))
  (if (`self.isAirborn`)
    (`self.ToggleAirborn` false)))

(fn `IsValidStab`
  (returns (IsValidStab :type Boolean) (SwordStabDistance :type "Float (double-precision)") (SwordVelocity :type "Float (double-precision)"))
  (bind _output_get (set `self.SocketPositionB` (`self.SocketPositionA`)))
  (bind _output_get_2 (set `self.SocketPositionA` (`SceneComponent.GetSocketLocation` (`self.SwordMesh`) "Collision_start")))
  (bind _returnvalue (`PrimitiveComponent.GetPhysicsLinearVelocity` (`self.SwordMesh`) "None"))
  (bind _returnvalue_2 (`KismetMathLibrary.Vector_Distance` _output_get_2 _output_get))
  (bind _returnvalue_3 (`KismetMathLibrary.VSizeSquared` _returnvalue))
  (return (and (>= _returnvalue_2 (`self.RequiredStabDistance`)) (> _returnvalue_3 (`self.RequiredStabVelocity`))) _returnvalue_2 _returnvalue_3))

(fn `IsValidSwing`
  (returns (IsValidSwing :type Boolean) (SwordSwingDistance :type "Float (double-precision)") (SwordVelocity :type "Float (double-precision)"))
  (bind _output_get (set `self.SocketPositionB` (`self.SocketPositionA`)))
  (bind _output_get_2 (set `self.SocketPositionA` (`SceneComponent.GetSocketLocation` (`self.SwordMesh`) "Collision_start")))
  (bind _returnvalue (`PrimitiveComponent.GetPhysicsLinearVelocity` (`self.SwordMesh`) "None"))
  (if (`self.isAirborn`)
    (bind _returnvalue_2 (`KismetMathLibrary.Vector_Distance` _output_get_2 _output_get))
    (bind _returnvalue_3 (`KismetMathLibrary.VSizeSquared` _returnvalue))
    (return true _returnvalue_2 _returnvalue_3)
    (else
      (return (and (>= _returnvalue_2 (`self.RequiredSwingDistance`)) (> _returnvalue_3 (`self.RequiredSwingVelocity`))) _returnvalue_2 _returnvalue_3))))

(fn `ReleaseSword`
  (bind _handcompref (`self.HandCompRef`))
  (`|ExecutionSequence`
    (:`then_0`
      (`PrimitiveComponent.SetEnableGravity` (`self.SwordMesh`) true)
      (bind _asvrpawn_main (cast `/Game/Transfusion/Blueprints/VRPawn_Main` (`ActorComponent.GetOwner` (`/Game/VRTemplate/Blueprints/GrabComponent.MotionControllerRef` (`self.GrabComponent`)))))
      (if (== (`MotionControllerComponent.MotionSource` (`self.HandParentRef`)) "LEFT")
        ;[1 1 1] Left Hand Release
        (`PhysicsHandleComponent.ReleaseComponent` (`/Game/Transfusion/Blueprints/VRPawn_Main.PhysicsHandleLeft` _asvrpawn_main))
        (else
          ;[1 1 1] Right Hand Release
          (`PhysicsHandleComponent.ReleaseComponent` (`/Game/Transfusion/Blueprints/VRPawn_Main.PhysicsHandleRight` _asvrpawn_main))))
      (`SceneComponent.K2_AttachToComponent` _handcompref (`self.HandParentRef`) "None" "SnapToTarget" "SnapToTarget" "SnapToTarget" true)
      (`SceneComponent.K2_SetRelativeTransform` _handcompref (`self.HandTransformRef`) false false)
      (set `self.HandCompRef` null)
      (set `self.HandParentRef` null)
      (set `self.HandTransformRef` (struct))
      (`KismetSystemLibrary.PrintString` "Released"))
    (:`then_1`
      (bind _returnvalue (`PrimitiveComponent.GetPhysicsLinearVelocity` (`self.SwordMesh`) "None"))
      (if (>= (`KismetMathLibrary.VSizeSquared` _returnvalue) 200000.0)
        (`self.ToggleAirborn` true)))))

(fn `SliceProceduralMesh`
  (params (SwingVelocity :type "Float (double-precision)") (OtherComponent :type "PrimitiveComponent Object Reference"))
  (bind _slashplane (`self.SlashPlane`))
  (bind _asprocedural_mesh_component (cast `ProceduralMeshComponent` OtherComponent))
  (bind _outotherhalfprocmesh (`KismetProceduralMeshLibrary.SliceProceduralMesh` _asprocedural_mesh_component (`SceneComponent.K2_GetComponentLocation` _slashplane) (`SceneComponent.GetUpVector` _slashplane) true "CreateNewSectionForCap" "/Game/Transfusion/Materials/Flesh.Flesh"))
  (`PrimitiveComponent.SetSimulatePhysics` (`local.OtherComponent`) true)
  (`PrimitiveComponent.SetSimulatePhysics` _outotherhalfprocmesh true)
  (set `ActorComponent.ComponentTags` (`|MakeArray` "Sliceable" :!type "Name") _outotherhalfprocmesh)
  (bind _returnvalue (`MagicLeapControllerFunctionLibrary.GetHandForMotionSource` (`MotionControllerComponent.MotionSource` (`/Game/VRTemplate/Blueprints/GrabComponent.MotionControllerRef` (`self.GrabComponent`)))))
  (`PlayerController.PlayHapticEffect` (`GameplayStatics.GetPlayerController` 0) "/Game/Transfusion/Haptics/SliceHapticEffect.SliceHapticEffect" _returnvalue (/ SwingVelocity (`self.RequiredSwingVelocity`)) false))

(fn `SliceTimer`
  (set `self.CanSlash` true))

(fn `StabTimer`
  (set `self.CanStab` true))

(fn `ToggleAirborn`
  (params (Airborn :type Boolean))
  (bind _slashplane (`self.SlashPlane`))
  (bind _swordmesh (`self.SwordMesh`))
  (bind _output_get (set `self.isAirborn` Airborn))
  (if _output_get
    (`SceneComponent.K2_SetRelativeLocation` _slashplane (`self.AirbornSlashPlanePosition`) false false)
    (`SceneComponent.SetRelativeScale3D` _slashplane (`self.AirbornSlashPlaneScale`))
    (`PrimitiveComponent.SetPhysicsAngularVelocityInDegrees` _swordmesh (* (`SceneComponent.GetRightVector` _swordmesh) 100000.0) true "None")
    (else
      (`SceneComponent.K2_SetRelativeLocation` _slashplane (`self.NormalSlashPlanePosition`) false false)
      (`SceneComponent.SetRelativeScale3D` _slashplane (`self.NormalSlashPlaneScale`)))))

(fn `UpdatePhysicsHandle`
  (bind _grabcomponent (`self.GrabComponent`))
  (bind _motioncontrollerref (`/Game/VRTemplate/Blueprints/GrabComponent.MotionControllerRef` _grabcomponent))
  (bind _returnvalue (`SceneComponent.K2_GetComponentLocation` _motioncontrollerref))
  (bind _returnvalue_2 (`KismetMathLibrary.ComposeRotators` (`KismetMathLibrary.NegateRotator` (`SceneComponent.RelativeRotation` _grabcomponent)) (`SceneComponent.K2_GetComponentRotation` _motioncontrollerref)))
  (bind _asvrpawn_main (cast `/Game/Transfusion/Blueprints/VRPawn_Main` (`ActorComponent.GetOwner` (`/Game/VRTemplate/Blueprints/GrabComponent.MotionControllerRef` (`self.GrabComponent`)))))
  (if (== (`MotionControllerComponent.MotionSource` (`self.HandParentRef`)) "LEFT")
    ;[1 1 1] Left Hand Update
    (`PhysicsHandleComponent.SetTargetLocationAndRotation` (`/Game/Transfusion/Blueprints/VRPawn_Main.PhysicsHandleLeft` _asvrpawn_main) _returnvalue _returnvalue_2)
    (else
      ;[1 1 1] Right Hand Update
      (`PhysicsHandleComponent.SetTargetLocationAndRotation` (`/Game/Transfusion/Blueprints/VRPawn_Main.PhysicsHandleRight` _asvrpawn_main) _returnvalue _returnvalue_2))))

(fn `UserConstructionScript`)