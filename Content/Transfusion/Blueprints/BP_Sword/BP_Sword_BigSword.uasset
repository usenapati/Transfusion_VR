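; BP_Sword_BigSword is a VR sword variant whose magic temporarily doubles its size.
; UseMagic slows the holding hand's physics handle interpolation on VRPawn_Main, quarters the required swing velocity and blocks further magic until a timer calls ResetBigSword to revert everything.
; A dynamic material lights the blade while magic is active.
; Going airborne adds spin around the mesh's right vector.
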(fn `ResetBigSword`
  (locals (NormalSwordSpeed :type "Float (double-precision)" :default 25.0))
  (bind _objectmesh (`self.ObjectMesh`))
  (bind _normalswordspeed (`local.NormalSwordSpeed`))
  (bind _lastmotioncontroller (`self.LastMotionController`))
  (`SceneComponent.SetWorldScale3D` _objectmesh (/ (`SceneComponent.K2_GetComponentScale` _objectmesh) 2.0))
  (bind _asvrpawn_main (cast `/Game/Transfusion/Blueprints/VRPawn_Main` (`ActorComponent.GetOwner` _lastmotioncontroller)))
  (if (== (`MotionControllerComponent.MotionSource` _lastmotioncontroller) "LEFT")
    (`PhysicsHandleComponent.SetInterpolationSpeed` (`/Game/Transfusion/Blueprints/VRPawn_Main.PhysicsHandleLeft` _asvrpawn_main) _normalswordspeed)
    (else
      (`PhysicsHandleComponent.SetInterpolationSpeed` (`/Game/Transfusion/Blueprints/VRPawn_Main.PhysicsHandleRight` _asvrpawn_main) _normalswordspeed)))
  (set `self.RequiredSwingVelocity` (* (`self.RequiredSwingVelocity`) 4.0))
  (set `self.MagicBlocked` false))

(fn `ToggleAirborn`
  (params (Airborn :type Boolean))
  (returns (IsAirborn :type Boolean))
  (locals (SpinSpeed :type "Float (double-precision)" :default 30000.0))
  (bind _objectmesh (`self.ObjectMesh`))
  (if Airborn
    (`PrimitiveComponent.SetPhysicsAngularVelocityInDegrees` _objectmesh (* (`SceneComponent.GetRightVector` _objectmesh) (`local.SpinSpeed`)) true "None")
    (return (`local.Airborn`))))

(fn `ToggleMagicActive`
  (params (Active :type Boolean))
  (bind _swordmaterial (`self.SwordMaterial`))
  (`parent.ToggleMagicActive` Active)
  (if Active
    (`MaterialInstanceDynamic.SetScalarParameterValue` _swordmaterial "BladeLightIntensity" 2.0)
    (else
      (`MaterialInstanceDynamic.SetScalarParameterValue` _swordmaterial "BladeLightIntensity" 0.0))))

(fn `UseMagic`
  (locals (BigSwordDuration :type "Float (double-precision)" :default 10.0) (SlowSwordSpeed :type "Float (double-precision)" :default 12.0))
  (bind _objectmesh (`self.ObjectMesh`))
  (bind _lastmotioncontroller (`self.LastMotionController`))
  (bind _slowswordspeed (`local.SlowSwordSpeed`))
  (bind _use_magic_ (`parent.UseMagic`))
  (if _use_magic_
    (`SceneComponent.SetWorldScale3D` _objectmesh (* (`SceneComponent.K2_GetComponentScale` _objectmesh) 2.0))
    (bind _asvrpawn_main (cast `/Game/Transfusion/Blueprints/VRPawn_Main` (`ActorComponent.GetOwner` _lastmotioncontroller)))
    (if (== (`MotionControllerComponent.MotionSource` _lastmotioncontroller) "LEFT")
      (`PhysicsHandleComponent.SetInterpolationSpeed` (`/Game/Transfusion/Blueprints/VRPawn_Main.PhysicsHandleLeft` _asvrpawn_main) _slowswordspeed)
      (else
        (`PhysicsHandleComponent.SetInterpolationSpeed` (`/Game/Transfusion/Blueprints/VRPawn_Main.PhysicsHandleRight` _asvrpawn_main) _slowswordspeed)))
    (set `self.RequiredSwingVelocity` (/ (`self.RequiredSwingVelocity`) 4.0))
    (set `self.MagicBlocked` true)
    (`KismetSystemLibrary.K2_SetTimer` null "ResetBigSword" (`local.BigSwordDuration`))))

(fn `UserConstructionScript`
  (`parent.UserConstructionScript`)
  (bind _returnvalue (`PrimitiveComponent.CreateDynamicMaterialInstance` (`self.ObjectMesh`) 0 null "None"))
  (set `self.SwordMaterial` _returnvalue))