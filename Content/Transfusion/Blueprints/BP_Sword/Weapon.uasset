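; Motion-controller sword that slashes, stabs and procedurally slices enemies.
; Slash and stab plane overlaps pick the hit type from component tags, then require enough per-tick socket travel and velocity (anti-waggle), waived for airborne slashes.
; Joint and body hits send damage through interface messages and fill a blood meter that enables magic and its light when full.
; Sliceable procedural meshes are cut along the slash plane into re-sliceable physics halves, with haptic feedback.
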(event `self.ReceiveTick`
  (params (DeltaSeconds :type "Float (single-precision)"))
  (`parent.ReceiveTick` DeltaSeconds)
  ;[1 1 1] Update Socket Tracking (Anti-Waggle)
  (set `self.SocketPositionPrev` (`self.SocketPositionCurrent`))
  (set `self.SocketPositionCurrent` (`SceneComponent.GetSocketLocation` (`self.ObjectMesh`) "Collision_start")))

(event `self.SlashPlane.OnComponentBeginOverlap`
  (params (OverlappedComponent :type "PrimitiveComponent Object Reference") (OtherActor :type "Actor Object Reference") (OtherComp :type "PrimitiveComponent Object Reference") (OtherBodyIndex :type Integer) (bFromSweep :type Boolean) (SweepResult :type "HitResult Structure (by ref)"))
  (bind _componenttags (`ActorComponent.ComponentTags` OtherComp))
  ;[1 1 1] Handle Slashing
  (bind (_isvalidslashtarget _slashtype) (`self.DecideSlashType` OtherActor _componenttags))
  (if _isvalidslashtarget
    (`/Engine/EditorBlueprintResources/StandardMacros.DoOnce` false :!label _label
      (:`Completed`
        (`self.DoSlash` _slashtype OtherActor OtherComp _componenttags SweepResult)))))

(event `self.SlashPlane.OnComponentEndOverlap`
  (params (OverlappedComponent :type "PrimitiveComponent Object Reference") (OtherActor :type "Actor Object Reference") (OtherComp :type "PrimitiveComponent Object Reference") (OtherBodyIndex :type Integer))
  ;[1 1 1] Handle Slashing
  (goto _label :!via `Reset`))

(event `self.StabPlane.OnComponentBeginOverlap`
  (params (OverlappedComponent :type "PrimitiveComponent Object Reference") (OtherActor :type "Actor Object Reference") (OtherComp :type "PrimitiveComponent Object Reference") (OtherBodyIndex :type Integer) (bFromSweep :type Boolean) (SweepResult :type "HitResult Structure (by ref)"))
  (bind _componenttags (`ActorComponent.ComponentTags` OtherComp))
  (bind _returnvalue (`KismetArrayLibrary.Array_Contains` _componenttags "Joint"))
  (bind _returnvalue_2 (`KismetArrayLibrary.Array_Contains` _componenttags "Body"))
  ;[1 1 1] Handle Stabbing
  (if (and (`KismetSystemLibrary.DoesImplementInterface` OtherActor "/Game/Transfusion/Blueprints/Interfaces/IEnemyInterface.IEnemyInterface_C") (`self.CanStab`) (or _returnvalue _returnvalue_2))
    (bind (_isvalidstab _swordstabdistance _swordvelocity) (`self.IsValidStab`))
    (if _isvalidstab
      (set `self.CanStab` false)
      (if _returnvalue
        (message `/Game/Transfusion/Blueprints/Interfaces/IEnemyInterface.Hit Joint` OtherActor 30 _swordstabdistance _swordvelocity _componenttags true SweepResult)
        (`self.AddBloodMeter` 30.0)
        (`KismetSystemLibrary.PrintString` "Damaged Enemy: STAB JOINT")
        (`KismetSystemLibrary.K2_SetTimerDelegate` (delegate `ResetStab`) 1.0 :!label _label_2)
        (elif _returnvalue_2
          (message `/Game/Transfusion/Blueprints/Interfaces/IEnemyInterface.Hit Body` OtherActor 20 _swordstabdistance _swordvelocity SweepResult)
          (`self.AddBloodMeter` 20.0)
          (`KismetSystemLibrary.PrintString` "Damaged Enemy: STAB BODY")
          (goto _label_2))))))

(event `ResetStab`
  ;[1 1 1] Handle Stabbing
  (set `self.CanStab` true))

(event `self.StabPlane.OnComponentEndOverlap`
  (params (OverlappedComponent :type "PrimitiveComponent Object Reference") (OtherActor :type "Actor Object Reference") (OtherComp :type "PrimitiveComponent Object Reference") (OtherBodyIndex :type Integer))
  ;[1 1 1] Handle Stabbing
)

(fn `AddBloodMeter`
  (params (Amount :type "Float (double-precision)"))
  (bind _bloodmetermax (`self.BloodMeterMax`))
  (bind _output_get (set `self.BloodMeter` (`KismetMathLibrary.FMin` (+ Amount (`self.BloodMeter`)) _bloodmetermax)))
  (if (>= _output_get _bloodmetermax)
    (`self.ToggleMagicActive` true)))

(fn `DecideSlashType`
  (params (OtherActor :type "Object Object Reference") (`Component Tags` :type "Array of Name (by ref)"))
  (returns (IsValidSlashTarget :type Boolean) (SlashType :type "/Game/Transfusion/Blueprints/BP_Sword/SlashType Enum"))
  (locals (returnSlashType :type "/Game/Transfusion/Blueprints/BP_Sword/SlashType Enum") (returnValidSlashTarget :type Boolean))
  ;[1 1 1] ProceduralSlice path
  (if (`KismetArrayLibrary.Array_Contains` `Component Tags` "Sliceable")
    (set `local.returnSlashType` "NewEnumerator2")
    ;[1 1 1] Valid Slash path
    (if (`self.CanSlash`) :!label _label
      (set `local.returnValidSlashTarget` true))
    (else
      ;[1 1 1] Joint Slash path
      (if (`KismetArrayLibrary.Array_Contains` `Component Tags` "Joint")
        (set `local.returnSlashType` "NewEnumerator1")
        (goto _label)
        (else
          ;[1 1 1] Body Slash path
          (if (`KismetArrayLibrary.Array_Contains` `Component Tags` "Body")
            (set `local.returnSlashType` "NewEnumerator0")
            (goto _label)
            (else
              _))))))
  (return (`local.returnValidSlashTarget`) (`local.returnSlashType`)))

(fn `DoSlash`
  (params (SlashType :type "/Game/Transfusion/Blueprints/BP_Sword/SlashType Enum" :default "NewEnumerator0") (`Other Actor` :type "Actor Object Reference") (OtherComponent :type "PrimitiveComponent Object Reference") (`Component Tags` :type "Array of Name (by ref)") (Hit :type "HitResult Structure"))
  (locals (SwordSwingDistance :type "Float (double-precision)") (SwordSwingVelocity :type "Float (double-precision)"))
  (bind _swordswingvelocity (`local.SwordSwingVelocity`))
  (bind (_isvalidswing _swordswingdistance _swordvelocity) (`self.IsValidSwing`))
  (if _isvalidswing
    (set `local.SwordSwingDistance` _swordswingdistance)
    (set `local.SwordSwingVelocity` _swordvelocity)
    (set `self.CanSlash` false)
    (switch `/Game/Transfusion/Blueprints/BP_Sword/SlashType` SlashType
      (:`NewEnumerator0`
        (message `/Game/Transfusion/Blueprints/Interfaces/IEnemyInterface.Hit Body` (`local.Other Actor`) 20 (`local.SwordSwingDistance`) (`local.SwordSwingVelocity`) Hit)
        (`self.AddBloodMeter` 20.0)
        (`KismetSystemLibrary.PrintString` "Damaged Enemy:  SLASH BODY"))
      (:`NewEnumerator1`
        (message `/Game/Transfusion/Blueprints/Interfaces/IEnemyInterface.Hit Joint` (`local.Other Actor`) 30 (`local.SwordSwingDistance`) (`local.SwordSwingVelocity`) (`local.Component Tags`) false Hit)
        (`self.AddBloodMeter` 30.0)
        (`KismetSystemLibrary.PrintString` "Damaged Enemy:  SLASH JOINT"))
      (:`NewEnumerator2`
        (message `/Game/Transfusion/Blueprints/Interfaces/IProceduralSliceInterface.BeforeSlice` (`local.Other Actor`) (`self.SlashPlane`) (`MotionControllerComponent.MotionSource` (`/Game/VRTemplate/Blueprints/GrabComponent.MotionControllerRef` (`self.GrabComponent`))) _swordswingvelocity)
        (`self.ProceduralSlice` _swordswingvelocity (`local.OtherComponent`))))
    (set `self.CanSlash` true)))

(fn `IsValidStab`
  (returns (IsValidStab :type Boolean) (SwordStabDistance :type "Float (double-precision)") (SwordVelocity :type "Float (double-precision)"))
  (locals (RequiredStabVelocity :type "Float (double-precision)" :default 40000.0) (RequiredStabDistance :type "Float (double-precision)" :default 0.0))
  (bind _returnvalue (`KismetMathLibrary.Vector_Distance` (`self.SocketPositionPrev`) (`self.SocketPositionCurrent`)))
  (bind _returnvalue_2 (`PrimitiveComponent.GetPhysicsLinearVelocity` (`self.ObjectMesh`) "None"))
  (bind _returnvalue_3 (`KismetMathLibrary.VSizeSquared` _returnvalue_2))
  (return (and (>= _returnvalue (`local.RequiredStabDistance`)) (> _returnvalue_3 (`local.RequiredStabVelocity`))) _returnvalue _returnvalue_3))

(fn `IsValidSwing`
  (returns (IsValidSwing :type Boolean) (SwordSwingDistance :type "Float (double-precision)") (SwordVelocity :type "Float (double-precision)"))
  (locals (RequiredSwingDistance :type "Float (double-precision)" :default 10.0) (RequiredSwingVelocity :type "Float (double-precision)" :default 400000.0))
  (bind _returnvalue (`KismetMathLibrary.Vector_Distance` (`self.SocketPositionPrev`) (`self.SocketPositionCurrent`)))
  (bind _returnvalue_2 (`PrimitiveComponent.GetPhysicsLinearVelocity` (`self.ObjectMesh`) "None"))
  (if (`self.isAirborn`)
    (bind _returnvalue_3 (`KismetMathLibrary.VSizeSquared` _returnvalue_2))
    (return true _returnvalue _returnvalue_3)
    (else
      (return (and (>= _returnvalue (`local.RequiredSwingDistance`)) (> _returnvalue_3 (`local.RequiredSwingVelocity`))) _returnvalue _returnvalue_3))))

(fn `ProceduralSlice`
  (params (SwingVelocity :type "Float (double-precision)") (OtherComponent :type "PrimitiveComponent Object Reference"))
  (locals (RequiredProceduralSwingVelocity :type "Float (double-precision)" :default 400000.0))
  (bind _slashplane (`self.SlashPlane`))
  (bind _asprocedural_mesh_component (cast `ProceduralMeshComponent` OtherComponent))
  (bind _outotherhalfprocmesh (`KismetProceduralMeshLibrary.SliceProceduralMesh` _asprocedural_mesh_component (`SceneComponent.K2_GetComponentLocation` _slashplane) (`SceneComponent.GetUpVector` _slashplane) true "CreateNewSectionForCap" "/Game/Transfusion/Materials/Flesh.Flesh"))
  (`PrimitiveComponent.SetSimulatePhysics` (`local.OtherComponent`) true)
  (`PrimitiveComponent.SetSimulatePhysics` _outotherhalfprocmesh true)
  (set `ActorComponent.ComponentTags` (`|MakeArray` "Sliceable" :!type "Name") _outotherhalfprocmesh)
  (bind _returnvalue (`MagicLeapControllerFunctionLibrary.GetHandForMotionSource` (`MotionControllerComponent.MotionSource` (`/Game/VRTemplate/Blueprints/GrabComponent.MotionControllerRef` (`self.GrabComponent`)))))
  (`PlayerController.PlayHapticEffect` (`GameplayStatics.GetPlayerController` 0) "/Game/VRTemplate/Haptics/SliceHapticEffect.SliceHapticEffect" _returnvalue (/ SwingVelocity (`local.RequiredProceduralSwingVelocity`)) false))

(fn `ToggleAirborn`
  (params (Airborn :type Boolean))
  (returns (IsAirborn :type Boolean))
  (locals (Rotation :type "Rotator Structure" :default (struct :`Pitch` 90.0)) (SpinSpeed :type "Float (double-precision)" :default 30000.0))
  (bind _objectmesh (`self.ObjectMesh`))
  (if Airborn
    (`PrimitiveComponent.SetPhysicsAngularVelocityInDegrees` _objectmesh (* (`SceneComponent.GetForwardVector` _objectmesh) (`local.SpinSpeed`)) true "None")
    (return (`local.Airborn`))))

(fn `ToggleMagicActive`
  (params (Active :type Boolean))
  (bind _pointlight (`self.PointLight`))
  (bind _output_get (set `self.IsMagicActive` Active))
  (if _output_get
    (`KismetSystemLibrary.PrintString` "Magic Active!")
    (`SceneComponent.SetVisibility` _pointlight true false)
    (else
      (`KismetSystemLibrary.PrintString` "Magic No Longer Active!")
      (`SceneComponent.SetVisibility` _pointlight false false))))

(fn `UseMagic`
  (if (not (`self.MagicBlocked`))
    (set `self.BloodMeter` 0.0)
    (`self.ToggleMagicActive` false)))

(fn `UserConstructionScript`
  (`parent.UserConstructionScript`))