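; BP_Kill_Shield is a shield Blueprint, filed with the sword Blueprints, whose only active logic gives its mesh a spin.
; ToggleAirborn zeroes ObjectMesh's world rotation, then adds angular velocity about its up vector, scaled by SpinSpeed, so physics drives the spin.
; Its branch condition is fixed to true, so the spin applies whatever Airborn holds, and that value is returned unchanged.
; The event graph holds only disabled default events.
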(fn `ToggleAirborn`
  (params (Airborn :type Boolean))
  (returns (IsAirborn :type Boolean))
  (locals (SpinSpeed :type "Float (double-precision)" :default 100000.0))
  (bind _objectmesh (`self.ObjectMesh`))
  (if true
    (`SceneComponent.K2_SetWorldRotation` :`self` (`self.ObjectMesh`))
    (`PrimitiveComponent.SetPhysicsAngularVelocityInDegrees` _objectmesh (* (`SceneComponent.GetUpVector` _objectmesh) (`local.SpinSpeed`)) true "None")
    (return (`local.Airborn`))))

(fn `UserConstructionScript`
  (`parent.UserConstructionScript`))