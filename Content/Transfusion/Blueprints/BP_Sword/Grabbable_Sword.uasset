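; Grabbable sword Blueprint that slices procedural meshes when it strikes them fast enough.
; A Plane component overlap, limited by a DoOnce until overlap ends, checks the velocity of the static mesh's attach parent against a required threshold.
; Hits above it cut along the Plane's location and up vector, capping with gold metal and simulating physics on the new half.
; Debug prints report physics state and velocity.
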(event `self.ReceiveActorBeginOverlap`
  (params (OtherActor :type "Actor Object Reference"))
  (`KismetSystemLibrary.PrintString` (`KismetStringLibrary.Conv_BoolToString` (`SceneComponent.IsSimulatingPhysics` (`SceneComponent.GetAttachParent` (`self.StaticMesh`)) "None"))))

(event `InputAction|GrabRight`
  (params (Key :type "Key Structure")))

(event `self.ReceiveBeginPlay`)

(event `self.Plane.OnComponentBeginOverlap`
  (params (OverlappedComponent :type "PrimitiveComponent Object Reference") (OtherActor :type "Actor Object Reference") (OtherComp :type "PrimitiveComponent Object Reference") (OtherBodyIndex :type Integer) (bFromSweep :type Boolean) (SweepResult :type "HitResult Structure (by ref)"))
  (bind _plane (`self.Plane`))
  (bind _returnvalue (`KismetMathLibrary.VSize` (`SceneComponent.GetComponentVelocity` (`SceneComponent.GetAttachParent` (`self.StaticMesh`)))))
  (`/Engine/EditorBlueprintResources/StandardMacros.DoOnce` false :!label _label
    (:`Completed`
      (`KismetSystemLibrary.PrintString` (`KismetStringLibrary.Conv_DoubleToString` _returnvalue))
      (if (> _returnvalue (`self.RequiredVelocity`))
        (bind _asprocedural_mesh_component (cast `ProceduralMeshComponent` OtherComp))
        (bind _outotherhalfprocmesh (`KismetProceduralMeshLibrary.SliceProceduralMesh` _asprocedural_mesh_component (`SceneComponent.K2_GetComponentLocation` _plane) (`SceneComponent.GetUpVector` _plane) true "CreateNewSectionForCap" "/Game/StarterContent/Materials/M_Metal_Gold.M_Metal_Gold"))
        (`PrimitiveComponent.SetSimulatePhysics` _outotherhalfprocmesh true)))))

(event `self.Plane.OnComponentEndOverlap`
  (params (OverlappedComponent :type "PrimitiveComponent Object Reference") (OtherActor :type "Actor Object Reference") (OtherComp :type "PrimitiveComponent Object Reference") (OtherBodyIndex :type Integer))
  (goto _label :!via `Reset`))

(fn `UserConstructionScript`)