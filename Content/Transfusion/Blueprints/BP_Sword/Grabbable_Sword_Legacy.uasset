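; Legacy grabbable sword that cuts procedural meshes when swung fast enough.
; A plane overlap, gated once per contact, compares the blade's squared physics velocity to a threshold, with a short timer as slice cooldown.
; A valid hit slices the mesh along the plane, caps it with a flesh material and simulates physics on the new half.
; Right-hand haptics scale with swing speed squared.
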(event `self.Plane.OnComponentBeginOverlap`
  (params (OverlappedComponent :type "PrimitiveComponent Object Reference") (OtherActor :type "Actor Object Reference") (OtherComp :type "PrimitiveComponent Object Reference") (OtherBodyIndex :type Integer) (bFromSweep :type Boolean) (SweepResult :type "HitResult Structure (by ref)"))
  (bind _plane (`self.Plane`))
  (`KismetSystemLibrary.PrintString` (`KismetSystemLibrary.GetDisplayName` OtherComp))
  (bind _returnvalue (`PrimitiveComponent.GetPhysicsLinearVelocity` (`self.StaticMesh`) "None"))
  (`/Engine/EditorBlueprintResources/StandardMacros.DoOnce` false :!label _label
    (:`Completed`
      (bind _returnvalue_2 (`KismetMathLibrary.VSizeSquared` _returnvalue))
      (`KismetSystemLibrary.PrintString` (`KismetStringLibrary.Conv_DoubleToString` _returnvalue_2))
      (if (and (> _returnvalue_2 (`self.RequiredVelocity`)) (`self.CanSlice`))
        (set `self.CanSlice` false)
        (`KismetSystemLibrary.K2_SetTimer` null "SliceTimer" 0.1)
        (bind _asprocedural_mesh_component (cast `ProceduralMeshComponent` OtherComp)
          (:`then`
            (bind _outotherhalfprocmesh (`KismetProceduralMeshLibrary.SliceProceduralMesh` _asprocedural_mesh_component (`SceneComponent.K2_GetComponentLocation` _plane) (`SceneComponent.GetUpVector` _plane) true "CreateNewSectionForCap" "/Game/Transfusion/Materials/Flesh.Flesh"))
            (`PlayerController.PlayHapticEffect` (`GameplayStatics.GetPlayerController` 0) "/Game/VRTemplate/Haptics/SliceHapticEffect.SliceHapticEffect" "Right" (/ _returnvalue_2 400000.0) false)
            (`PrimitiveComponent.SetSimulatePhysics` _outotherhalfprocmesh true))
          (:`CastFailed`
            (`KismetSystemLibrary.PrintString` "FAILED TO CAST TO PROCEDURAL MESH")))))))

(event `self.Plane.OnComponentEndOverlap`
  (params (OverlappedComponent :type "PrimitiveComponent Object Reference") (OtherActor :type "Actor Object Reference") (OtherComp :type "PrimitiveComponent Object Reference") (OtherBodyIndex :type Integer))
  (goto _label :!via `Reset`))

(fn `SliceTimer`
  (set `self.CanSlice` true))

(fn `UserConstructionScript`)