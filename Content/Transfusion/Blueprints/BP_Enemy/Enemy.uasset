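; Enemy actor that swaps its skeletal mesh for a physics-simulated procedural mesh when hit by a sword.
; The construction script copies the static mesh component into the procedural mesh with collision.
; On the first overlap with Grabbable_Sword, it reveals that mesh, enables physics and destroys the skeletal mesh, guarded by a MeshSpawned flag.
; It prints "CUTTING" but performs no slice itself.
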(event `self.ReceiveActorBeginOverlap`
  (params (OtherActor :type "Actor Object Reference"))
  (bind _proceduralmesh (`self.ProceduralMesh`))
  (if (and (== (`GameplayStatics.GetObjectClass` OtherActor) "/Game/Transfusion/Blueprints/BP_Sword/Grabbable_Sword.Grabbable_Sword_C") (not (`self.MeshSpawned`)))
    (`KismetSystemLibrary.PrintString` "CUTTING")
    (`SceneComponent.SetVisibility` _proceduralmesh true false)
    (`SceneComponent.SetHiddenInGame` _proceduralmesh false false)
    (`PrimitiveComponent.SetSimulatePhysics` _proceduralmesh true)
    (`ActorComponent.K2_DestroyComponent` (`self.SkeletalMesh`))
    (set `self.MeshSpawned` true)))

(fn `UserConstructionScript`
  (`KismetProceduralMeshLibrary.CopyProceduralMeshFromStaticMeshComponent` (`self.StaticMesh`) 0 (`self.ProceduralMesh`) true))