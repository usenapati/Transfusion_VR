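; Sword-wielding lizard enemy that damages the VR player through overlaps on its sword slot.
; Inherits setup, attack selection, hit reactions, dismemberment and death from its parent.
; Triggered attacks play a randomly selected montage, setting an upper-body flag for all but the kick.
; Montage start and notifies toggle the damage window, which allows one player hit scaled by the attack multiplier before closing.
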(event `self.ReceiveBeginPlay`
  ;[1 1 1] Parent Functions
  ;;[1 1 1] Enemy Initialization
  (`parent.ReceiveBeginPlay`))

(event `self.SwordSlot.OnComponentBeginOverlap`
  (params (OverlappedComponent :type "PrimitiveComponent Object Reference") (OtherActor :type "Actor Object Reference") (OtherComp :type "PrimitiveComponent Object Reference") (OtherBodyIndex :type Integer) (bFromSweep :type Boolean) (SweepResult :type "HitResult Structure (by ref)"))
  ;[1 1 1] Damage Player
  (if (and (`self.CanDamage`) (`self.IsAlive`))
    (bind _asvrpawn_main (cast `/Game/Transfusion/Blueprints/VRPawn_Main` OtherActor))
    (`/Game/Transfusion/Blueprints/VRPawn_Main.TakeDamage` _asvrpawn_main (* (`self.BaseDamage`) (`self.CurrentAttackMultiplier`)))
    (set `self.CanDamage` false)))

(event `self.ReceiveTick`
  (params (DeltaSeconds :type "Float (single-precision)"))
  ;[1 1 1] Parent Functions
  ;;[1 1 1] Tick
  (`parent.ReceiveTick` DeltaSeconds))

(event `/Game/Transfusion/Blueprints/Interfaces/IEnemyInterface.Apply Damage`
  (params (Damage :type Integer))
  ;[1 1 1] Parent Functions
  ;;[1 1 1] Interface Functions
  ;;;[1 1 1] Dismemberment Events
  (`parent.Apply Damage` Damage))

(event `/Game/Transfusion/Blueprints/Interfaces/IEnemyInterface.Kill Enemy`
  ;[1 1 1] Parent Functions
  ;;[1 1 1] Interface Functions
  ;;;[1 1 1] Animation Events
  (`parent.Kill Enemy`))

(event `/Game/Transfusion/Blueprints/Interfaces/IEnemyAIInterface.SelectAttack`
  ;[1 1 1] Parent Functions
  ;;[1 1 1] Interface Functions
  ;;;[1 1 1] Attacks
  (`parent.SelectAttack`))

(event `Handle Sword Attack Animations`
  ;[1 1 1] Attack Animations
  (bind (_anim_montage _no_montage) (`self.RandomSelectAttack` (`self.SelectedAttackType`)))
  (if _no_montage
    (`self.Select Attack`)
    (else
      (bind _output_get (set `self.SelectedAttackMontage` _anim_montage))
      ;;[1 1 1] Play Montage
      (set `self.Upper Body?` (not (== _output_get "/Game/Transfusion/Animations/LizAnim/Sword_Attacks/M_Sword_And_Shield_Kick.M_Sword_And_Shield_Kick")))
      (bind _notifyname (`|PlayMontage` (`self.Mesh`) (`self.SelectedAttackMontage`))
        (:`then`
          (`self.Toggle Damage` true :!label _label))
        (:`OnCompleted`
          (set `self.Upper Body?` false)
          (`GameplayStatics.PlaySoundAtLocation` "/Game/Transfusion/Audio/Effects/LizardAttack_Cue.LizardAttack_Cue" (`self.K2_GetActorLocation`) (struct) 1.0 1.0 0.0 null null null)
          (`self.Toggle Damage` false)
          (set `self.CurrentAttackMultiplier` 1.0))
        (:`OnNotifyBegin`
          (if (== _notifyname "StartDamage")
            (goto _label)
            (elif (== _notifyname "StopDamage")
              (`self.Toggle Damage` false))))))))

(event `/Game/Transfusion/Blueprints/Interfaces/IEnemyAIInterface.TriggerAttack`
  ;[1 1 1] Parent Functions
  ;;[1 1 1] Interface Functions
  ;;;[1 1 1] Attacks
  (`self.Handle Sword Attack Animations`))

(event `/Game/Transfusion/Blueprints/Interfaces/IEnemyInterface.Sever Limb`
  (params (`Gore Part` :type "Actor Class Reference") (`Bone(s)` :type "Array of Name (by ref)"))
  ;[1 1 1] Parent Functions
  ;;[1 1 1] Interface Functions
  ;;;[1 1 1] Dismemberment Events
  (`parent.Sever Limb` `Gore Part` `Bone(s)`))

(event `/Game/Transfusion/Blueprints/Interfaces/IEnemyInterface.Hit Body`
  (params (Damage :type Integer) (AttackWidth :type "Float (single-precision)") (AttackSpeed :type "Float (single-precision)") (Hit :type "HitResult Structure"))
  ;[1 1 1] Parent Functions
  ;;[1 1 1] Interface Functions
  ;;;[1 1 1] Dismemberment Events
  (`parent.Hit Body` Damage AttackWidth AttackSpeed Hit))

(event `/Game/Transfusion/Blueprints/Interfaces/IEnemyInterface.Hit Joint`
  (params (Damage :type Integer) (AttackWidth :type "Float (single-precision)") (AttackSpeed :type "Float (single-precision)") (CollisionTags :type "Array of Name (by ref)") (IsStab :type Boolean) (Hit :type "HitResult Structure"))
  ;[1 1 1] Parent Functions
  ;;[1 1 1] Interface Functions
  ;;;[1 1 1] Dismemberment Events
  (`parent.Hit Joint` Damage AttackWidth AttackSpeed CollisionTags IsStab Hit))

(fn `Is Alive`
  (returns (`Is Alive` :type Boolean))
  (return (`self.IsAlive`)))

(fn `UserConstructionScript`
  (`parent.UserConstructionScript`))