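; Sliceable enemy character that swaps its skeletal mesh for a physics-simulated procedural mesh when cut.
; The construction script copies a static mesh into the procedural mesh with collision, then destroys the static mesh component.
; Overlap with a Grabbable_Sword or a Slice call reveals that mesh and destroys the skeletal one, once via MeshSpawned.
; Only Slice also disables capsule collision; neither path cuts geometry here.
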(event `self.ReceiveActorBeginOverlap`
  (params (OtherActor :type "Actor Object Reference"))
  (bind _proceduralmesh (`self.ProceduralMesh`))
  (if (and (== (`GameplayStatics.GetObjectClass` OtherActor) "/Game/Transfusion/Blueprints/BP_Sword/Grabbable_Sword.Grabbable_Sword_C") (not (`self.MeshSpawned`)))
    (`KismetSystemLibrary.PrintString` "CUTTING")
    (`SceneComponent.SetVisibility` _proceduralmesh true false)
    (`SceneComponent.SetHiddenInGame` _proceduralmesh false false)
    (`PrimitiveComponent.SetSimulatePhysics` _proceduralmesh true)
    (`ActorComponent.K2_DestroyComponent` (`self.Mesh`))
    (set `self.MeshSpawned` true)))

(fn `Slice`
  (bind _proceduralmesh (`self.ProceduralMesh`))
  (if (not (`self.MeshSpawned`))
    (`KismetSystemLibrary.PrintString` "CUTTING")
    (`SceneComponent.SetVisibility` _proceduralmesh true false)
    (`SceneComponent.SetHiddenInGame` _proceduralmesh false false)
    (`PrimitiveComponent.SetSimulatePhysics` _proceduralmesh true)
    (`ActorComponent.K2_DestroyComponent` (`self.Mesh`))
    (`PrimitiveComponent.SetCollisionEnabled` (`self.CapsuleComponent`) "NoCollision")
    (set `self.MeshSpawned` true)))

(fn `UserConstructionScript`
  (bind _staticmesh (`self.StaticMesh`))
  (`parent.UserConstructionScript`)
  (`KismetProceduralMeshLibrary.CopyProceduralMeshFromStaticMeshComponent` _staticmesh 0 (`self.ProceduralMesh`) true)
  (`ActorComponent.K2_DestroyComponent` _staticmesh))