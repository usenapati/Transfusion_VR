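; Lizard enemy for VR sword combat that registers with the combat director, targets the player and can be dismembered.
; Randomly chosen light, heavy or combo montages use notifies to toggle sword damage.
; Joint hits passing width and speed thresholds sever limbs by hiding bones, spawning gore actors and briefly slowing time.
; Zero health, decapitation or losing both legs triggers ragdoll, then delayed removal updates the director and game mode.
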(event `self.ReceiveBeginPlay`
  (bind _returnvalue (`KismetMathLibrary.Conv_IntToDouble` (`self.MaxHealth`)))
  ;[1 1 1] Enemy Initialization
  (bind _returnvalue_2 (`GameplayStatics.GetActorOfClass` "/Game/Transfusion/Blueprints/VRPawn_Main.VRPawn_Main_C"))
  (`/Engine/EditorBlueprintResources/StandardMacros.IsValid` _returnvalue_2
    (:`Is Valid`
      (set `self.CurrentTarget` _returnvalue_2))
    (:`Is Not Valid`
      (bind _returnvalue_3 (`GameplayStatics.GetActorOfClass` "/Game/Transfusion/Blueprints/Legacy/BP_VRDummy/BP_VRDummy.BP_VRDummy_C"))
      (set `self.CurrentTarget` _returnvalue_3)))
  (bind _asenemy_health_widget (cast `/Game/Transfusion/Widgets/Enemy_Health_Widget` (`WidgetComponent.GetUserWidgetObject` (`self.HealthWidget`))))
  (bind _output_get (set `self.HealthWidgetREF` _asenemy_health_widget))
  (set `/Game/Transfusion/Widgets/Enemy_Health_Widget.Health` _returnvalue _output_get)
  (set `/Game/Transfusion/Widgets/Enemy_Health_Widget.MaxHealth` _returnvalue _output_get)
  ;;[1 1 1] Add to Combat Director
  (bind _returnvalue_4 (`GameplayStatics.GetActorOfClass` "/Game/Transfusion/Blueprints/EnemyManagers/BP_CombatDirector.BP_CombatDirector_C"))
  (bind _output_get_2 (set `self.CombatDirectorREF` _returnvalue_4))
  (`/Engine/EditorBlueprintResources/StandardMacros.IncrementInt` (`/Game/Transfusion/Blueprints/EnemyManagers/BP_CombatDirector.Enemy Alive` _output_get_2)
    (:`  `
      (`KismetArrayLibrary.Array_Add` (`/Game/Transfusion/Blueprints/EnemyManagers/BP_CombatDirector.EnemyList` _output_get_2) self)
      (`/Game/Transfusion/Blueprints/EnemyManagers/BP_CombatDirector.AddDebugWidgets` _output_get_2 self)
      (bind _asenemy_controller (cast `/Game/Transfusion/BehaviorTree/EnemyController` (`self.GetController`)))
      (`BlueprintMapLibrary.Map_Add` (`/Game/Transfusion/Blueprints/EnemyManagers/BP_CombatDirector.EnemyStates` _output_get_2) self (`/Game/Transfusion/BehaviorTree/EnemyController.CurrentState` _asenemy_controller)))))

(event `self.ReceiveTick`
  (params (DeltaSeconds :type "Float (single-precision)"))
  (`self.Initial Animation`)
  (if (`self.IsDead`)
    (`KismetSystemLibrary.Delay` 4.0 :!label _label)
    (`self.Kill Enemy Lizard`)
    (elif (`self.SlicedNeck`)
      (goto _label)
      (elif (`NavMovementComponent.IsFalling` (`self.CharacterMovement`))
        _))))

(event `/Game/Transfusion/Blueprints/Interfaces/IEnemyInterface.Apply Damage`
  (params (Damage :type Integer))
  ;[1 1 1] Dismemberment Events
  ;;[1 1 1] Damage Enemy
  (`self.Damage Enemy` Damage))

(event `/Game/Transfusion/Blueprints/Interfaces/IEnemyInterface.Kill Enemy`
  ;[1 1 1] Animation Events
  ;;[1 1 1] Death
  (`self.Enable Ragdoll`))

(event `/Game/Transfusion/Blueprints/Interfaces/IEnemyAIInterface.SelectAttack`
  ;[1 1 1] AI Events
  ;;[1 1 1] Attacks
  (`self.Select Attack`))

(event `/Game/Transfusion/Blueprints/Interfaces/IEnemyAIInterface.TriggerAttack`
  ;[1 1 1] AI Events
  ;;[1 1 1] Attacks
  (`self.HandleAttackAnimations`))

(event `/Game/Transfusion/Blueprints/Interfaces/IEnemyInterface.Sever Limb`
  (params (`Gore Part` :type "Actor Class Reference") (`Bone(s)` :type "Array of Name (by ref)"))
  ;[1 1 1] Dismemberment Events
  ;;[1 1 1] Sever Limb
  (`self.Sever Enemy Limb` `Gore Part` `Bone(s)`))

(event `/Game/Transfusion/Blueprints/Interfaces/IEnemyInterface.Hit Body`
  (params (Damage :type Integer) (AttackWidth :type "Float (single-precision)") (AttackSpeed :type "Float (single-precision)") (Hit :type "HitResult Structure"))
  ;[1 1 1] Dismemberment Events
  ;;[1 1 1] Hit Body
  (`self.Hit Enemy Body` Damage AttackWidth AttackSpeed Hit))

(event `self.SwordSlot.OnComponentBeginOverlap`
  (params (OverlappedComponent :type "PrimitiveComponent Object Reference") (OtherActor :type "Actor Object Reference") (OtherComp :type "PrimitiveComponent Object Reference") (OtherBodyIndex :type Integer) (bFromSweep :type Boolean) (SweepResult :type "HitResult Structure (by ref)"))
  ;[1 1 1] AI Events
  ;;[1 1 1] Damage Player
  (if (`self.CanDamage`)
    (bind _asvrpawn_main (cast `/Game/Transfusion/Blueprints/VRPawn_Main` OtherActor))
    (`/Game/Transfusion/Blueprints/VRPawn_Main.TakeDamage` _asvrpawn_main (* (`self.BaseDamage`) (`self.CurrentAttackMultiplier`)))
    (set `self.CanDamage` false)))

(event `/Game/Transfusion/Blueprints/Interfaces/IEnemyInterface.Hit Joint`
  (params (Damage :type Integer) (AttackWidth :type "Float (single-precision)") (AttackSpeed :type "Float (single-precision)") (CollisionTags :type "Array of Name (by ref)") (IsStab :type Boolean) (Hit :type "HitResult Structure"))
  ;[1 1 1] Dismemberment Events
  ;;[1 1 1] Hit Joint
  (`self.Hit Enemy Joint` Damage AttackWidth AttackSpeed CollisionTags IsStab Hit))

(event `HandleAttackAnimations`
  (bind _lightattacks (`self.LightAttacks`))
  (bind _heavyattacks (`self.HeavyAttacks`))
  (bind _comboattacks (`self.ComboAttacks`))
  ;[1 1 1] Attack Animations
  (switch `name` (`self.SelectedAttack`)
    (:`LightAttack`
      (set `self.SelectedAttackMontage` (`|GetArrayItem` _lightattacks (`KismetMathLibrary.RandomIntegerInRange` 0 (`KismetArrayLibrary.Array_Length` _lightattacks)))))
    (:`HeavyAttack`
      (set `self.SelectedAttackMontage` (`|GetArrayItem` _heavyattacks (`KismetMathLibrary.RandomIntegerInRange` 0 (`KismetArrayLibrary.Array_Length` _heavyattacks)))))
    (:`ComboAttack`
      (set `self.SelectedAttackMontage` (`|GetArrayItem` _comboattacks (`KismetMathLibrary.RandomIntegerInRange` 0 (`KismetArrayLibrary.Array_Length` _comboattacks))))))
  ;;[1 1 1] Play Montage
  (set `self.Upper Body?` true)
  (bind _notifyname (`|PlayMontage` (`self.Mesh`) (`self.SelectedAttackMontage`))
    (:`then`
      (`self.Toggle Damage` true :!label _label_2))
    (:`OnCompleted`
      (set `self.Upper Body?` false)
      (`GameplayStatics.PlaySoundAtLocation` "/Game/Transfusion/Audio/Effects/LizardAttack_Cue.LizardAttack_Cue" (`self.K2_GetActorLocation`) (struct) 1.0 1.0 0.0 null null null)
      (`self.Toggle Damage` false)
      (set `self.CurrentAttackMultiplier` 1.0))
    (:`OnNotifyBegin`
      (if (== _notifyname "StartDamage")
        (goto _label_2)
        (elif (== _notifyname "StopDamage")
          (`self.Toggle Damage` false))))))

(fn `Add to Combo and Powerup Meter`
  (params (ComboToAdd :type Integer) (PowerupMeterToAdd :type Integer))
  (bind _asvrgame_mode (cast `/Game/Transfusion/Blueprints/Globals/VRGameMode` (`GameplayStatics.GetGameMode`)))
  (`/Game/Transfusion/Blueprints/Globals/VRGameMode.AddCombo` _asvrgame_mode ComboToAdd)
  (bind _asvrpawn_main (cast `/Game/Transfusion/Blueprints/VRPawn_Main` (`GameplayStatics.GetPlayerPawn` 0)))
  (`/Game/Transfusion/Blueprints/VRPawn_Main.AddToPowerupMeter` _asvrpawn_main PowerupMeterToAdd))

(fn `Damage Enemy`
  (params (Damage :type Integer))
  (bind _returnvalue (`self.K2_GetActorLocation`))
  (bind _output_get (set `self.Health` (- (`self.Health`) Damage)))
  (set `/Game/Transfusion/Widgets/Enemy_Health_Widget.Health` (`KismetMathLibrary.Conv_IntToDouble` _output_get) (`self.HealthWidgetREF`))
  (if (<= _output_get 0)
    (`self.Enable Ragdoll`))
  (`self.Add to Combo and Powerup Meter` 5 10)
  (set `self.IsHit` true)
  (`KismetSystemLibrary.K2_SetTimer` null "Reset IsHit" (`self.Invincibility Duration`))
  (`GameplayStatics.PlaySoundAtLocation` "/Game/Transfusion/Audio/Source/MixKit/MetalHit.MetalHit" _returnvalue (struct) 1.0 1.0 0.0 null null null)
  (`GameplayStatics.PlaySoundAtLocation` "/Game/Transfusion/Audio/Effects/LizardHurt_Cue.LizardHurt_Cue" _returnvalue (struct) 1.0 1.0 0.0 null null null))

(fn `Decide Hit`
  (params (GorePart :type "Actor Class Reference") (SlicedPart :type Boolean) (`Bone(s)` :type "Array of Name") (AttackWidth :type "Float (double-precision)") (AttackSpeed :type "Float (double-precision)") (IsStab :type Boolean))
  (returns (DisableHitBoxes :type Boolean))
  (if SlicedPart
    (`KismetSystemLibrary.PrintString` "ALREADY SLICED")
    (return false)
    (else
      (if true
        (if (and (> AttackWidth (`self.RequiredStabWidth`)) (> AttackSpeed (`self.RequiredStabVelocity`)))
          _
          (else
            (return false)))
        (elif (and (> AttackWidth (`self.RequiredSwingWidth`)) (> AttackSpeed (`self.RequiredSwingVelocity`)))
          _
          (else
            (return false))))
      (`self.Sever Enemy Limb` GorePart `Bone(s)`)
      (`KismetSystemLibrary.PrintString` "SEVERED LIMB")
      (return true))))

(fn `Detect Body Part`
  (params (CollisionTags :type "Array of Name"))
  (returns (GorePart :type "Actor Class Reference") (SlicedPart :type Boolean) (`Bone(s)` :type "Array of Name") (`Joint(s)` :type "Array of SphereComponent Object Reference") (`Hit Box(es)` :type "Array of CapsuleComponent Object Reference"))
  (switch `name` (`|GetArrayItem` CollisionTags 1)
    (:`LeftShoulder`
      ;[1 1 1] Arms
      ;;[1 1 1] Left Arm
      (return "/Game/Transfusion/Blueprints/BP_Enemy/LizardEnemy_Base/BP_SlicedLizardBase_LeftArm.BP_SlicedLizardBase_LeftArm_C" (`self.SlicedLeftArm`) (`|MakeArray` (`self.upper_arm_L`)) (`|MakeArray` (`self.Shoulder_LCollider`)) (`|MakeArray` (`self.Hand_LHitbox`) (`self.ForeArm_LHitbox`) (`self.UpperArm_LHitbox`))))
    (:`RightShoulder`
      ;;[1 1 1] Right Arm
      (return "/Game/Transfusion/Blueprints/BP_Enemy/LizardEnemy_Base/BP_SlicedLizardBase_RightArm.BP_SlicedLizardBase_RightArm_C" (`self.SlicedRightArm`) (`|MakeArray` (`self.upper_arm_R`)) (`|MakeArray` (`self.Shoulder_RCollider`)) (`|MakeArray` (`self.Hand_RHitbox`) (`self.ForeArm_RHitbox`) (`self.UpperArm_RHitbox`))))
    (:`LeftHip`
      ;[1 1 1] Legs
      ;;[1 1 1] Left Leg
      (return "/Game/Transfusion/Blueprints/BP_Enemy/LizardEnemy_Base/BP_SlicedLizardBase_LeftLeg.BP_SlicedLizardBase_LeftLeg_C" (`self.SlicedLeftLeg`) (`|MakeArray` (`self.thigh_L`)) (`|MakeArray` (`self.Hip_LCollider`)) (`|MakeArray` (`self.Foot_LHitbox`) (`self.Calf_LHitbox`) (`self.Thigh_LHitbox`))))
    (:`RightHip`
      ;;[1 1 1] Right Leg
      (return "/Game/Transfusion/Blueprints/BP_Enemy/LizardEnemy_Base/BP_SlicedLizardBase_RightLeg.BP_SlicedLizardBase_RightLeg_C" (`self.SlicedRightLeg`) (`|MakeArray` (`self.thigh_R`)) (`|MakeArray` (`self.Hip_RCollider`)) (`|MakeArray` (`self.Foot_RHitbox`) (`self.Calf_RHitbox`) (`self.Thigh_RHitbox`))))
    (:`Neck`
      ;[1 1 1] Neck
      (return "/Game/Transfusion/Blueprints/BP_Enemy/LizardEnemy_Base/BP_SlicedLizardBase_Head.BP_SlicedLizardBase_Head_C" (`self.SlicedNeck`) (`|MakeArray` (`self.neck`)) (`|MakeArray` (`self.NeckCollider`)) (`|MakeArray` (`self.HeadHitBox`))))))

(fn `Disable Hitboxes`
  (params (`Joint(s)` :type "Array of SphereComponent Object Reference") (`HItBox(es)` :type "Array of CapsuleComponent Object Reference"))
  (for _array_element `Joint(s)`
    (`PrimitiveComponent.SetCollisionEnabled` _array_element "NoCollision"))
  (for _array_element_2 `HItBox(es)`
    (`PrimitiveComponent.SetCollisionEnabled` _array_element_2 "NoCollision")))

(fn `Enable Ragdoll`
  (`/Engine/EditorBlueprintResources/StandardMacros.DoOnce` false
    (:`Completed`
      ;[1 1 1] Not Ragdolling
      (for _array_element (`SceneComponent.GetChildrenComponents` (`self.Mesh`) true)
        (bind _asskeletal_mesh_component (cast `SkeletalMeshComponent` _array_element)
          (:`then`
            (`PrimitiveComponent.SetCollisionProfileName` _asskeletal_mesh_component "Ragdoll" false))
          (:`CastFailed`
            (bind _ascapsule_collision (cast `CapsuleComponent` _array_element))
            (`PrimitiveComponent.SetCollisionProfileName` _ascapsule_collision "OverlapAllDynamic" false))))
      (set `self.Upper Body?` false)
      (`/Game/Transfusion/Blueprints/Components/PhysicalAnimComponent.EnterRagdoll` (`self.PhysicalAnimComponent`))
      (set `self.IsDead` true))))

(fn `Hit Enemy Body`
  (params (Damage :type Integer) (`Attack Width` :type "Float (double-precision)") (`Attack Speed` :type "Float (double-precision)") (Hit :type "HitResult Structure"))
  (`self.Damage Enemy` Damage)
  (`/Game/Transfusion/Blueprints/Components/PhysicalAnimComponent.HitReaction` (`self.GetComponentByClass` "/Game/Transfusion/Blueprints/Components/PhysicalAnimComponent.PhysicalAnimComponent_C") Hit `Attack Speed`))

(fn `Hit Enemy Joint`
  (params (Damage :type Integer) (`Attack Width` :type "Float (double-precision)") (`Attack Speed` :type "Float (double-precision)") (`Collision Tags` :type "Array of Name") (`Is Stab` :type Boolean) (Hit :type "HitResult Structure"))
  (bind (_gorepart _slicedpart _bone_s_ _joint_s_ _hit_box_es_) (`self.Detect Body Part` `Collision Tags`))
  (bind _disablehitboxes (`self.Decide Hit` _gorepart _slicedpart _bone_s_ `Attack Width` `Attack Speed` `Is Stab`))
  (if _disablehitboxes
    (`self.Disable Hitboxes` _joint_s_ _hit_box_es_)
    (`self.Damage Enemy` 40)
    (else
      (`self.Damage Enemy` Damage)))
  (`/Game/Transfusion/Blueprints/Components/PhysicalAnimComponent.HitReaction` (`self.GetComponentByClass` "/Game/Transfusion/Blueprints/Components/PhysicalAnimComponent.PhysicalAnimComponent_C") Hit `Attack Speed`))

(fn `Initial Animation`
  (if (== (`NavMovementComponent.IsFalling` (`self.CharacterMovement`)) (`self.HasLanded`))
    (set `self.HasLanded` true)
    (`self.PlayAnimMontage` "/Game/Transfusion/Animations/LizAnim/M_Sword_And_Shield_Power_Up.M_Sword_And_Shield_Power_Up")))

(fn `Kill Enemy Lizard`
  (bind _returnvalue (`self.K2_GetActorLocation`))
  (bind _combatdirectorref (`self.CombatDirectorREF`))
  (bind _asvrgame_mode (cast `/Game/Transfusion/Blueprints/Globals/VRGameMode` (`GameplayStatics.GetGameMode`)))
  (`/Game/Transfusion/Blueprints/Globals/VRGameMode.UpdateCounter` _asvrgame_mode)
  (`/Engine/EditorBlueprintResources/StandardMacros.DecrementInt` (`/Game/Transfusion/Blueprints/EnemyManagers/BP_CombatDirector.Enemy Alive` (`self.CombatDirectorREF`))
    (:`  `
      (`KismetArrayLibrary.Array_RemoveItem` (`/Game/Transfusion/Blueprints/EnemyManagers/BP_CombatDirector.EnemyList` _combatdirectorref) self)
      (`BlueprintMapLibrary.Map_Remove` (`/Game/Transfusion/Blueprints/EnemyManagers/BP_CombatDirector.EnemyGrading` _combatdirectorref) self)
      (`BlueprintMapLibrary.Map_Remove` (`/Game/Transfusion/Blueprints/EnemyManagers/BP_CombatDirector.EnemyWidgets` _combatdirectorref) self)
      (`GameplayStatics.PlaySoundAtLocation` "/Game/Transfusion/Audio/Effects/CriticalHit_Cue.CriticalHit_Cue" _returnvalue (struct) 1.0 1.0 0.0 null null null)
      (`GameplayStatics.PlaySoundAtLocation` "/Game/Transfusion/Audio/Effects/LizardHiss_Cue.LizardHiss_Cue" _returnvalue (struct) 1.0 1.0 0.0 null null null)
      (if (`self.TimeDilated`)
        (`self.ResetTimeDilation`))
      (`self.K2_DestroyActor`))))

(fn `Reset IsHit`)

(fn `ResetTimeDilation`
  (set `self.TimeDilated` false)
  (`GameplayStatics.SetGlobalTimeDilation` 1.0))

(fn `Select Attack`
  (locals (SelectedAttackString :type String))
  (bind _output_get (set `self.AttackHeuristic` (`KismetMathLibrary.RandomFloatInRange` 0.0 1.0)))
  (if (< _output_get 0.333333)
    (bind _output_get_2 (set `self.SelectedAttack` "LightAttack"))
    ;[1 1 1] Debug
    (set `local.SelectedAttackString` (`KismetStringLibrary.Concat_StrStr` "Selected: " (`KismetStringLibrary.Conv_NameToString` _output_get_2)))
    (elif (< _output_get 0.666667)
      (bind _output_get_3 (set `self.SelectedAttack` "HeavyAttack"))
      (set `self.CurrentAttackMultiplier` (`self.HeavyAttackMultiplier`))
      (set `local.SelectedAttackString` (`KismetStringLibrary.Concat_StrStr` "Selected: " (`KismetStringLibrary.Conv_NameToString` _output_get_3)))
      (else
        (bind _output_get_4 (set `self.SelectedAttack` "ComboAttack"))
        (set `self.CurrentAttackMultiplier` (`self.ComboAttackMultiplier`))
        (set `local.SelectedAttackString` (`KismetStringLibrary.Concat_StrStr` "Selected: " (`KismetStringLibrary.Conv_NameToString` _output_get_4))))))
  (if (`self.DebugText`)
    (`KismetSystemLibrary.PrintString` (`local.SelectedAttackString`)))
  (`/Game/Transfusion/Blueprints/Interfaces/IEnemyAIInterface.TriggerAttack`))

(fn `Sever Enemy Limb`
  (params (`Gore Part` :type "Actor Class Reference") (`Bone(s)` :type "Array of Name"))
  (locals (Skip :type Boolean) (TimeDilationDuration :type "Float (double-precision)" :default 0.2))
  (bind _output (`|GetArrayItem` `Bone(s)`))
  (bind (_returnvalue_x _returnvalue_y _returnvalue_z) (`KismetMathLibrary.BreakVector` (`SceneComponent.GetSocketLocation` (`self.Mesh`) _output)))
  (set `local.Skip` true)
  (for _array_element `Bone(s)`
    (bind _returnvalue (`SkinnedMeshComponent.IsBoneHiddenByName` (`self.Mesh`) _array_element))
    (if (not _returnvalue)
      (set `local.Skip` false)))
  (if (not (`local.Skip`))
    (for _array_element_2 (`local.Bone(s)`)
      (`SkinnedMeshComponent.HideBoneByName` (`self.Mesh`) _array_element_2 "PBO_None")
      (`self.Update Sliced Vars By Bone Name` _array_element_2))
    (bind _returnvalue_2 (`|SpawnActorFromClass` (`local.Gore Part`) (`KismetMathLibrary.MakeTransform` (`KismetMathLibrary.MakeVector` _returnvalue_x _returnvalue_y (- _returnvalue_z 100.0))) "Undefined" "OverrideRootScale" null null))
    ;[1 1 1] Simulate Physics Toggle?
    (`PrimitiveComponent.AddImpulse` (`self.GetComponentByClass` _returnvalue_2 "/Script/Engine.SkeletalMeshComponent") (`KismetMathLibrary.MakeVector` 500.0 -500.0 500.0) (`|GetArrayItem` (`local.Bone(s)`)) true)
    (`KismetSystemLibrary.PrintString` (`KismetStringLibrary.Concat_StrStr` "SLICED :: " (`KismetSystemLibrary.GetClassDisplayName` (`local.Gore Part`))) true true (struct :`R` 0.008464 :`G` 0.052599 :`B` 0.8125 :`A` 1.0))
    (`GameplayStatics.PlaySoundAtLocation` "/Game/Transfusion/Audio/Effects/DismembermentHit_Cue.DismembermentHit_Cue" (`SceneComponent.GetSocketLocation` (`self.Mesh`) _output) (struct) 1.0 1.0 0.0 null null null)
    (`GameplayStatics.PlaySoundAtLocation` "/Game/Transfusion/Audio/Effects/LizardHurt_Cue.LizardHurt_Cue" (`self.K2_GetActorLocation`) (struct) 1.0 1.0 0.0 null null null)
    (`GameplayStatics.SpawnEmitterAttached` "/Game/Transfusion/VFX/PS_BloodSpurt.PS_BloodSpurt" (`self.Mesh`) _output (0.0 0.0 0.0) (struct) (1.0 1.0 1.0) "SnapToTarget")
    (if (== (`GameplayStatics.GetGlobalTimeDilation`) 1.0)
      (if (== (`|GetArrayItem` (`local.Bone(s)`)) "neck")
        (set `local.TimeDilationDuration` 0.2)
        (else
          (set `local.TimeDilationDuration` 0.05)))
      (`GameplayStatics.SetGlobalTimeDilation` 0.2)
      (set `self.TimeDilated` true)
      (`KismetSystemLibrary.K2_SetTimer` null "ResetTimeDilation" (`local.TimeDilationDuration`)))))

(fn `Toggle Damage`
  (params (CanDamage :type Boolean))
  (if (not (`self.SlicedRightArm`))
    (set `self.CanDamage` CanDamage)))

(fn `Update Sliced Vars By Bone Name`
  (params (`Bone Name` :type Name))
  (switch `name` `Bone Name`
    (:`neck`
      (set `self.SlicedNeck` true)
      (`self.Enable Ragdoll`))
    (:`thigh_R`
      (set `self.SlicedRightLeg` true)
      (if (and (`self.SlicedRightLeg`) (`self.SlicedLeftLeg`)) :!label _label
        (`self.Enable Ragdoll`)))
    (:`thigh_L`
      (set `self.SlicedLeftLeg` true)
      (goto _label))
    (:`upper_arm_R`
      (set `self.SlicedRightArm` true)
      (`SceneComponent.SetVisibility` (`self.SwordSlot`) false false))
    (:`upper_arm_L`
      (set `self.SlicedLeftArm` true))))

(fn `UserConstructionScript`
  ;[1 1 1] Construct Master Pose
  (`SkinnedMeshComponent.SetLeaderPoseComponent` (`self.RightArm`) (`self.Mesh`) false)
  (`SkinnedMeshComponent.SetLeaderPoseComponent` (`self.LeftArm`) (`self.Mesh`) false)
  (`SkinnedMeshComponent.SetLeaderPoseComponent` (`self.RightLeg`) (`self.Mesh`) false)
  (`SkinnedMeshComponent.SetLeaderPoseComponent` (`self.LeftLeg`) (`self.Mesh`) false)
  (`SkinnedMeshComponent.SetLeaderPoseComponent` (`self.Tail`) (`self.Mesh`) false)
  (`SkinnedMeshComponent.SetLeaderPoseComponent` (`self.Torso`) (`self.Mesh`) false))