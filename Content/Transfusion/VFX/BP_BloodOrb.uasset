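; Blood orb VFX actor that homes in on the player and is absorbed on contact.
; Each Tick it teleports to a position interpolated from its effect's location toward the player pawn's root, giving an eased pull.
; When its sphere overlaps the VR pawn, it plays a drop sound at the player, deactivates the effect and destroys itself.
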(event `self.ReceiveBeginPlay`)

(event `self.Sphere.OnComponentBeginOverlap`
  (params (OverlappedComponent :type "PrimitiveComponent Object Reference") (OtherActor :type "Actor Object Reference") (OtherComp :type "PrimitiveComponent Object Reference") (OtherBodyIndex :type Integer) (bFromSweep :type Boolean) (SweepResult :type "HitResult Structure (by ref)"))
  (bind _asvrpawn_main (cast `/Game/Transfusion/Blueprints/VRPawn_Main` OtherActor))
  (`GameplayStatics.PlaySoundAtLocation` "/Game/Transfusion/Audio/Source/drop.drop" (`SceneComponent.K2_GetComponentLocation` (`Actor.RootComponent` (`GameplayStatics.GetPlayerPawn` 0))) (struct) 1.0 1.0 0.0 null null null)
  (`ActorComponent.Deactivate` (`self.Effect`))
  (`self.K2_DestroyActor`))

(event `self.ReceiveTick`
  (params (DeltaSeconds :type "Float (single-precision)"))
  (`self.K2_TeleportTo` (`KismetMathLibrary.VInterpTo` (`SceneComponent.K2_GetComponentLocation` (`self.Effect`)) (`SceneComponent.K2_GetComponentLocation` (`Actor.RootComponent` (`GameplayStatics.GetPlayerPawn` 0))) DeltaSeconds 2.0)))

(fn `UserConstructionScript`)