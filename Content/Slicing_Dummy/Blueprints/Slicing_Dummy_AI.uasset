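; VR melee enemy dummy that registers with CombatDirector, attacks the player with a sword and can lose its arms.
; Per-body-part hitboxes apply damage from valid BP_Sword swings, with brief invincibility, feeding the health widget and combo/powerup meters.
; Below a health threshold, shoulder colliders sever arms by hiding bones on the master-pose modular body and launching spawned gore actors.
; Elbow cuts and gate-based dismemberment are unused.
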(event `Attack`
  (set `self.Upper Body?` true)
  (`|PlayMontage` (`self.Mesh`) "/Game/Slicing_Dummy/Animations/Attack/Standing_Melee_Attack_Horizontal_Montage.Standing_Melee_Attack_Horizontal_Montage"
    (:`then`
      (`KismetSystemLibrary.Delay` 4.0)
      (set `self.Upper Body?` false))))

(event `self.ReceiveTick`
  (params (DeltaSeconds :type "Float (single-precision)"))
  (if (<= (`self.Health`) 0)
    (`self.KillDummy`)))

(event `self.Sphere.OnComponentBeginOverlap`
  (params (OverlappedComponent :type "PrimitiveComponent Object Reference") (OtherActor :type "Actor Object Reference") (OtherComp :type "PrimitiveComponent Object Reference") (OtherBodyIndex :type Integer) (bFromSweep :type Boolean) (SweepResult :type "HitResult Structure (by ref)"))
  ;[1 1 1] Update Enemy Healthbar
  (cast `/Game/Transfusion/Blueprints/BP_Sword/BP_Sword` OtherActor)
  (`SceneComponent.SetVisibility` (`self.HealthWidget`) true false))

(event `self.ReceiveBeginPlay`
  (bind _returnvalue (`GameplayStatics.GetActorOfClass` "/Game/Transfusion/Blueprints/VRPawn.VRPawn_C"))
  (set `self.CurrentTarget` _returnvalue)
  (bind _asenemy_health_widget (cast `/Game/Transfusion/Widgets/Enemy_Health_Widget` (`WidgetComponent.GetUserWidgetObject` (`self.HealthWidget`))))
  (bind _output_get (set `self.HealthWidgetREF` _asenemy_health_widget))
  (set `/Game/Transfusion/Widgets/Enemy_Health_Widget.Health` (`KismetMathLibrary.Conv_IntToDouble` (`self.MaxHealth`)) _output_get)
  (bind _returnvalue_2 (`GameplayStatics.GetActorOfClass` "/Game/Transfusion/BehaviorTree/CombatDirector.CombatDirector_C"))
  (bind _output_get_2 (set `self.CombatDirectorREF` _returnvalue_2))
  (`/Engine/EditorBlueprintResources/StandardMacros.IncrementInt` (`/Game/Transfusion/BehaviorTree/CombatDirector.Enemy Alive` _output_get_2)
    (:`  `
      (`KismetArrayLibrary.Array_Add` (`/Game/Transfusion/BehaviorTree/CombatDirector.EnemyList` _output_get_2) self)
      (`/Game/Transfusion/BehaviorTree/CombatDirector.AddDebugWidgets` _output_get_2 self))))

(event `self.Sphere.OnComponentEndOverlap`
  (params (OverlappedComponent :type "PrimitiveComponent Object Reference") (OtherActor :type "Actor Object Reference") (OtherComp :type "PrimitiveComponent Object Reference") (OtherBodyIndex :type Integer))
  ;[1 1 1] Update Enemy Healthbar
  (cast `/Game/Transfusion/Blueprints/BP_Sword/BP_Sword` OtherActor)
  (`SceneComponent.SetVisibility` (`self.HealthWidget`) false false))

(event `self.RightForearmHitBox.OnComponentBeginOverlap`
  (params (OverlappedComponent :type "PrimitiveComponent Object Reference") (OtherActor :type "Actor Object Reference") (OtherComp :type "PrimitiveComponent Object Reference") (OtherBodyIndex :type Integer) (bFromSweep :type Boolean) (SweepResult :type "HitResult Structure (by ref)"))
  ;[1 1 1] Enemy Hit Detection
  (bind _asbp_sword (cast `/Game/Transfusion/Blueprints/BP_Sword/BP_Sword` OtherActor))
  (`self.Hit Enemy` _asbp_sword 5))

(event `self.RightShoulderCollider.OnComponentBeginOverlap`
  (params (OverlappedComponent :type "PrimitiveComponent Object Reference") (OtherActor :type "Actor Object Reference") (OtherComp :type "PrimitiveComponent Object Reference") (OtherBodyIndex :type Integer) (bFromSweep :type Boolean) (SweepResult :type "HitResult Structure (by ref)"))
  ;[1 1 1] Dismemberment System - Current
  ;;[1 1 1] Right Arm Dismemberment
  (bind _disablehitboxes (`self.Joint Hit` OtherComp "/Game/Slicing_Dummy/Blueprints/Slicing_RightArm.Slicing_RightArm_C" (`self.SlicedRightArm`) 75 (`|MakeArray` (`self.UpperArm_R`) (`self.Forearm_R`))))
  (if _disablehitboxes
    (`self.Disable HitBoxes` (`|MakeArray` (`self.RightShoulderCollider`) (`self.RightElbowCollider`)) (`|MakeArray` (`self.RightArmHitBox`) (`self.RightForearmHitBox`)))
    (`ActorComponent.K2_DestroyComponent` (`self.Sword`))))

(event `self.RightCalfHitBox.OnComponentBeginOverlap`
  (params (OverlappedComponent :type "PrimitiveComponent Object Reference") (OtherActor :type "Actor Object Reference") (OtherComp :type "PrimitiveComponent Object Reference") (OtherBodyIndex :type Integer) (bFromSweep :type Boolean) (SweepResult :type "HitResult Structure (by ref)"))
  ;[1 1 1] Enemy Hit Detection
  (bind _asbp_sword (cast `/Game/Transfusion/Blueprints/BP_Sword/BP_Sword` OtherActor))
  (`self.Hit Enemy` _asbp_sword 5))

(event `CloseLeftArmGate`
  (bind _slicedleftarm (`self.SlicedLeftArm`))
  (bind _forearm_l (`self.Forearm_L`))
  (bind _array (`|MakeArray` (`self.UpperArm_L`) _forearm_l))
  ;[1 1 1] DEPRECATED
  ;;[1 1 1] Left Arm Dismembermen - NOT USED
  (`/Engine/EditorBlueprintResources/StandardMacros.Gate` false :!via `Close`
    (:`Exit`
      (if _slicedleftarm
        (if (and (`self.SlicedLeftArm`) (`self.SlicedLeftForearm`))
          (`self.Sever Limb` "/Game/Slicing_Dummy/Blueprints/Slicing_LeftUpperArm.Slicing_LeftUpperArm_C" _array)
          (else
            (`self.Sever Limb` "/Game/Slicing_Dummy/Blueprints/Slicing_LeftArm.Slicing_LeftArm_C" _array)))
        (`self.CloseLeftArmGate`)
        (else
          (if (and (not _slicedleftarm) (`self.SlicedLeftForearm`))
            (`self.Sever Limb` "/Game/Slicing_Dummy/Blueprints/Slicing_LeftForearm.Slicing_LeftForearm_C" (`|MakeArray` _forearm_l))))))))

(event `self.RightFootHitBox.OnComponentBeginOverlap`
  (params (OverlappedComponent :type "PrimitiveComponent Object Reference") (OtherActor :type "Actor Object Reference") (OtherComp :type "PrimitiveComponent Object Reference") (OtherBodyIndex :type Integer) (bFromSweep :type Boolean) (SweepResult :type "HitResult Structure (by ref)"))
  ;[1 1 1] Enemy Hit Detection
  (bind _asbp_sword (cast `/Game/Transfusion/Blueprints/BP_Sword/BP_Sword` OtherActor))
  (`self.Hit Enemy` _asbp_sword 1))

(event `self.LeftShoulderCollider.OnComponentBeginOverlap`
  (params (OverlappedComponent :type "PrimitiveComponent Object Reference") (OtherActor :type "Actor Object Reference") (OtherComp :type "PrimitiveComponent Object Reference") (OtherBodyIndex :type Integer) (bFromSweep :type Boolean) (SweepResult :type "HitResult Structure (by ref)"))
  ;[1 1 1] Dismemberment System - Current
  ;;[1 1 1] Left Arm Dismemberment
  (bind _disablehitboxes (`self.Joint Hit` OtherComp "/Game/Slicing_Dummy/Blueprints/Slicing_LeftArm.Slicing_LeftArm_C" (`self.SlicedLeftArm`) 75 (`|MakeArray` (`self.UpperArm_L`) (`self.Forearm_L`))))
  (if _disablehitboxes
    (`self.Disable HitBoxes` (`|MakeArray` (`self.LeftShoulderCollider`) (`self.LeftElbowCollider`)) (`|MakeArray` (`self.LeftArmHitBox`) (`self.LefttForearmHitBox`)))))

(event `self.RightThighHitBox.OnComponentBeginOverlap`
  (params (OverlappedComponent :type "PrimitiveComponent Object Reference") (OtherActor :type "Actor Object Reference") (OtherComp :type "PrimitiveComponent Object Reference") (OtherBodyIndex :type Integer) (bFromSweep :type Boolean) (SweepResult :type "HitResult Structure (by ref)"))
  ;[1 1 1] Enemy Hit Detection
  (bind _asbp_sword (cast `/Game/Transfusion/Blueprints/BP_Sword/BP_Sword` OtherActor))
  (`self.Hit Enemy` _asbp_sword 5))

(event `self.LeftCalfHitBox.OnComponentBeginOverlap`
  (params (OverlappedComponent :type "PrimitiveComponent Object Reference") (OtherActor :type "Actor Object Reference") (OtherComp :type "PrimitiveComponent Object Reference") (OtherBodyIndex :type Integer) (bFromSweep :type Boolean) (SweepResult :type "HitResult Structure (by ref)"))
  ;[1 1 1] Enemy Hit Detection
  (bind _asbp_sword (cast `/Game/Transfusion/Blueprints/BP_Sword/BP_Sword` OtherActor))
  (`self.Hit Enemy` _asbp_sword 5))

(event `CloseRightArmGate`
  (bind _forearm_r (`self.Forearm_R`))
  (bind _slicedrightarm (`self.SlicedRightArm`))
  (bind _array (`|MakeArray` (`self.UpperArm_R`) _forearm_r))
  ;[1 1 1] DEPRECATED
  ;;[1 1 1] Right Arm Dismemberment - NOT USED
  (`/Engine/EditorBlueprintResources/StandardMacros.Gate` false :!via `Close`
    (:`Exit`
      (if _slicedrightarm
        (if (and (`self.SlicedRightArm`) (`self.SlicedRightForearm`))
          (`self.Sever Limb` "/Game/Slicing_Dummy/Blueprints/Slicing_LeftUpperArm.Slicing_LeftUpperArm_C" _array)
          (else
            (`self.Sever Limb` "/Game/Slicing_Dummy/Blueprints/Slicing_RightArm.Slicing_RightArm_C" _array)))
        (`self.CloseRightArmGate`)
        (else
          (if (and (not _slicedrightarm) (`self.SlicedRightForearm`))
            (`self.Sever Limb` "/Game/Slicing_Dummy/Blueprints/Slicing_LeftForearm.Slicing_LeftForearm_C" (`|MakeArray` _forearm_r))))))))

(event `self.RightElbowCollider.OnComponentBeginOverlap`
  (params (OverlappedComponent :type "PrimitiveComponent Object Reference") (OtherActor :type "Actor Object Reference") (OtherComp :type "PrimitiveComponent Object Reference") (OtherBodyIndex :type Integer) (bFromSweep :type Boolean) (SweepResult :type "HitResult Structure (by ref)"))
  ;[1 1 1] Right Forearm Dismemberment
)

(event `self.LeftFootHitBox.OnComponentBeginOverlap`
  (params (OverlappedComponent :type "PrimitiveComponent Object Reference") (OtherActor :type "Actor Object Reference") (OtherComp :type "PrimitiveComponent Object Reference") (OtherBodyIndex :type Integer) (bFromSweep :type Boolean) (SweepResult :type "HitResult Structure (by ref)"))
  ;[1 1 1] Enemy Hit Detection
  (bind _asbp_sword (cast `/Game/Transfusion/Blueprints/BP_Sword/BP_Sword` OtherActor))
  (`self.Hit Enemy` _asbp_sword 1))

(event `self.PelvisHitBox.OnComponentBeginOverlap`
  (params (OverlappedComponent :type "PrimitiveComponent Object Reference") (OtherActor :type "Actor Object Reference") (OtherComp :type "PrimitiveComponent Object Reference") (OtherBodyIndex :type Integer) (bFromSweep :type Boolean) (SweepResult :type "HitResult Structure (by ref)"))
  ;[1 1 1] Enemy Hit Detection
  (bind _asbp_sword (cast `/Game/Transfusion/Blueprints/BP_Sword/BP_Sword` OtherActor))
  (`self.Hit Enemy` _asbp_sword 10))

(event `self.LeftElbowCollider.OnComponentBeginOverlap`
  (params (OverlappedComponent :type "PrimitiveComponent Object Reference") (OtherActor :type "Actor Object Reference") (OtherComp :type "PrimitiveComponent Object Reference") (OtherBodyIndex :type Integer) (bFromSweep :type Boolean) (SweepResult :type "HitResult Structure (by ref)"))
  ;[1 1 1] Left Forearm Dismemberment
)

(event `self.LeftThighHitBox.OnComponentBeginOverlap`
  (params (OverlappedComponent :type "PrimitiveComponent Object Reference") (OtherActor :type "Actor Object Reference") (OtherComp :type "PrimitiveComponent Object Reference") (OtherBodyIndex :type Integer) (bFromSweep :type Boolean) (SweepResult :type "HitResult Structure (by ref)"))
  ;[1 1 1] Enemy Hit Detection
  (bind _asbp_sword (cast `/Game/Transfusion/Blueprints/BP_Sword/BP_Sword` OtherActor))
  (`self.Hit Enemy` _asbp_sword 5))

(event `self.RightArmHitBox.OnComponentBeginOverlap`
  (params (OverlappedComponent :type "PrimitiveComponent Object Reference") (OtherActor :type "Actor Object Reference") (OtherComp :type "PrimitiveComponent Object Reference") (OtherBodyIndex :type Integer) (bFromSweep :type Boolean) (SweepResult :type "HitResult Structure (by ref)"))
  ;[1 1 1] Enemy Hit Detection
  (bind _asbp_sword (cast `/Game/Transfusion/Blueprints/BP_Sword/BP_Sword` OtherActor))
  (`self.Hit Enemy` _asbp_sword 5))

(event `self.LefttForearmHitBox.OnComponentBeginOverlap`
  (params (OverlappedComponent :type "PrimitiveComponent Object Reference") (OtherActor :type "Actor Object Reference") (OtherComp :type "PrimitiveComponent Object Reference") (OtherBodyIndex :type Integer) (bFromSweep :type Boolean) (SweepResult :type "HitResult Structure (by ref)"))
  ;[1 1 1] Enemy Hit Detection
  (bind _asbp_sword (cast `/Game/Transfusion/Blueprints/BP_Sword/BP_Sword` OtherActor))
  (`self.Hit Enemy` _asbp_sword 5))

(event `self.LeftArmHitBox.OnComponentBeginOverlap`
  (params (OverlappedComponent :type "PrimitiveComponent Object Reference") (OtherActor :type "Actor Object Reference") (OtherComp :type "PrimitiveComponent Object Reference") (OtherBodyIndex :type Integer) (bFromSweep :type Boolean) (SweepResult :type "HitResult Structure (by ref)"))
  ;[1 1 1] Enemy Hit Detection
  (bind _asbp_sword (cast `/Game/Transfusion/Blueprints/BP_Sword/BP_Sword` OtherActor))
  (`self.Hit Enemy` _asbp_sword 5))

(event `self.TorsoHitBox.OnComponentBeginOverlap`
  (params (OverlappedComponent :type "PrimitiveComponent Object Reference") (OtherActor :type "Actor Object Reference") (OtherComp :type "PrimitiveComponent Object Reference") (OtherBodyIndex :type Integer) (bFromSweep :type Boolean) (SweepResult :type "HitResult Structure (by ref)"))
  ;[1 1 1] Enemy Hit Detection
  (bind _asbp_sword (cast `/Game/Transfusion/Blueprints/BP_Sword/BP_Sword` OtherActor))
  (`self.Hit Enemy` _asbp_sword 10))

(event `self.HeadHitBox.OnComponentBeginOverlap`
  (params (OverlappedComponent :type "PrimitiveComponent Object Reference") (OtherActor :type "Actor Object Reference") (OtherComp :type "PrimitiveComponent Object Reference") (OtherBodyIndex :type Integer) (bFromSweep :type Boolean) (SweepResult :type "HitResult Structure (by ref)"))
  ;[1 1 1] Enemy Hit Detection
  (bind _asbp_sword (cast `/Game/Transfusion/Blueprints/BP_Sword/BP_Sword` OtherActor))
  (`self.Hit Enemy` _asbp_sword 5))

(event `self.Sword.OnComponentEndOverlap`
  (params (OverlappedComponent :type "PrimitiveComponent Object Reference") (OtherActor :type "Actor Object Reference") (OtherComp :type "PrimitiveComponent Object Reference") (OtherBodyIndex :type Integer))
  ;[1 1 1] Need to turn off collider
  (bind _asvrpawn (cast `/Game/Transfusion/Blueprints/VRPawn` OtherActor))
  (if (`self.Upper Body?`)
    (`/Game/Transfusion/Blueprints/VRPawn.TakeDamage` _asvrpawn 10.0)))

(fn `Add to Combo and Powerup Meter`
  (params (ComboToAdd :type Integer) (PowerupMeterToAdd :type Integer))
  (bind _asvrgame_mode (cast `/Game/VRTemplate/Blueprints/VRGameMode` (`GameplayStatics.GetGameMode`)))
  (`/Game/VRTemplate/Blueprints/VRGameMode.AddCombo` _asvrgame_mode ComboToAdd)
  (bind _asvrpawn (cast `/Game/Transfusion/Blueprints/VRPawn` (`GameplayStatics.GetPlayerPawn` 0)))
  (`/Game/Transfusion/Blueprints/VRPawn.AddToPowerupMeter` _asvrpawn PowerupMeterToAdd))

(fn `Disable HitBoxes`
  (params (`Joint(s)` :type "Array of SphereComponent Object Reference") (`HitBoxe(s)` :type "Array of CapsuleComponent Object Reference"))
  (for _array_element `Joint(s)`
    (`PrimitiveComponent.SetCollisionEnabled` _array_element "NoCollision"))
  (for _array_element_2 `HitBoxe(s)`
    (`PrimitiveComponent.SetCollisionEnabled` _array_element_2 "NoCollision")))

(fn `Hit Enemy`
  (params (Sword :type "/Game/Transfusion/Blueprints/BP_Sword/BP_Sword Object Reference") (Damage :type Integer))
  (if (not (`self.IsHit`))
    (bind (_swordswingdistance _isvalidswing) (`/Game/Transfusion/Blueprints/BP_Sword/BP_Sword.IsValidSwing` Sword))
    (if _isvalidswing
      (bind _output_get (set `self.Health` (- (`self.Health`) Damage)))
      (set `/Game/Transfusion/Widgets/Enemy_Health_Widget.Health` (`KismetMathLibrary.Conv_IntToDouble` _output_get) (`self.HealthWidgetREF`))
      (`self.Add to Combo and Powerup Meter` 5 10)
      (set `self.IsHit` true)
      (`KismetSystemLibrary.K2_SetTimer` null "Reset IsHit" (`self.InvincibilityDuration`)))))

(fn `Joint Hit`
  (params (Actor :type "ActorComponent Object Reference") (GorePart :type "Actor Class Reference") (SlicePart :type Boolean) (RequiredHealth :type Integer) (`Bone(S)` :type "Array of Name"))
  (returns (DisableHitBoxes :type Boolean))
  (locals (SlicedPart :type Boolean :default true))
  (if (<= (`self.Health`) RequiredHealth)
    (bind _asbp_sword (cast `/Game/Transfusion/Blueprints/BP_Sword/BP_Sword` (`ActorComponent.GetOwner` Actor))
      (:`then`
        (if SlicePart
          (`KismetSystemLibrary.PrintString` "ALREADY SLICED")
          (return false)
          (else
            (bind (_swordswingdistance _isvalidswing) (`/Game/Transfusion/Blueprints/BP_Sword/BP_Sword.IsValidSwing` _asbp_sword))
            (if _isvalidswing
              (`self.Sever Limb` GorePart `Bone(S)`)
              (set `local.SlicedPart` SlicePart)
              (`KismetSystemLibrary.PrintString` "SEVERED LIMB")
              (return true)
              (else
                (`KismetSystemLibrary.PrintString` "SWING WAS NOT VALID")
                (`self.Add to Combo and Powerup Meter` 10 20)
                (return false))))))
      (:`CastFailed`
        (return false)))
    (else
      (return false))))

(fn `KillDummy`
  (bind _combatdirectorref (`self.CombatDirectorREF`))
  (`self.PlayAnimMontage` "/Game/Slicing_Dummy/Animations/Damage/Dying_Anim.Dying_Anim")
  (`/Engine/EditorBlueprintResources/StandardMacros.DecrementInt` (`/Game/Transfusion/BehaviorTree/CombatDirector.Enemy Alive` (`self.CombatDirectorREF`))
    (:`  `
      (`KismetArrayLibrary.Array_RemoveItem` (`/Game/Transfusion/BehaviorTree/CombatDirector.EnemyList` _combatdirectorref) self)
      (`BlueprintMapLibrary.Map_Remove` (`/Game/Transfusion/BehaviorTree/CombatDirector.EnemyGrading` _combatdirectorref) self)
      (`BlueprintMapLibrary.Map_Remove` (`/Game/Transfusion/BehaviorTree/CombatDirector.EnemyWidgets` _combatdirectorref) self)
      (`self.K2_DestroyActor`))))

(fn `Reset IsHit`
  (set `self.IsHit` false))

(fn `Sever Limb`
  (params (GorePart :type "Actor Class Reference") (`Bone(s)` :type "Array of Name"))
  (locals (Skip :type Boolean))
  (bind (_returnvalue_x _returnvalue_y _returnvalue_z) (`KismetMathLibrary.BreakVector` (`SceneComponent.GetSocketLocation` (`self.Mesh`) (`|GetArrayItem` `Bone(s)`))))
  (set `local.Skip` true)
  (for _array_element `Bone(s)`
    (bind _returnvalue (`SkinnedMeshComponent.IsBoneHiddenByName` (`self.Mesh`) _array_element))
    (if (not _returnvalue)
      (set `local.Skip` false)))
  (if (not (`local.Skip`))
    (for _array_element_2 (`local.Bone(s)`)
      (`SkinnedMeshComponent.HideBoneByName` (`self.Mesh`) _array_element_2 "PBO_None"))
    (bind _returnvalue_2 (`|SpawnActorFromClass` (`local.GorePart`) (`KismetMathLibrary.MakeTransform` (`KismetMathLibrary.MakeVector` _returnvalue_x _returnvalue_y (- _returnvalue_z 100.0))) "Undefined" "OverrideRootScale" null null))
    (`PrimitiveComponent.AddImpulse` (`self.GetComponentByClass` _returnvalue_2 "/Script/Engine.SkeletalMeshComponent") (`KismetMathLibrary.MakeVector` 500.0 -500.0 500.0) (`|GetArrayItem` (`local.Bone(s)`)) true)
    (`KismetSystemLibrary.PrintString` (`KismetStringLibrary.Concat_StrStr` "SLICED:: " (`KismetSystemLibrary.GetClassDisplayName` (`local.GorePart`))) true true (struct :`R` 0.008464 :`G` 0.052599 :`B` 0.8125 :`A` 1.0))))

(fn `Update Walk Speed`
  (params (NewWalkSpeed :type "Float (double-precision)"))
  (set `CharacterMovementComponent.MaxWalkSpeed` NewWalkSpeed (`self.CharacterMovement`)))

(fn `UserConstructionScript`
  (`SkinnedMeshComponent.SetLeaderPoseComponent` (`self.Torso`) (`self.Mesh`) false)
  (`SkinnedMeshComponent.SetLeaderPoseComponent` (`self.LeftArm`) (`self.Mesh`) false)
  (`SkinnedMeshComponent.SetLeaderPoseComponent` (`self.LeftForearm`) (`self.Mesh`) false)
  (`SkinnedMeshComponent.SetLeaderPoseComponent` (`self.RightArm`) (`self.Mesh`) false)
  (`SkinnedMeshComponent.SetLeaderPoseComponent` (`self.RightForearm`) (`self.Mesh`) false)
  (`SkinnedMeshComponent.SetLeaderPoseComponent` (`self.Pelvis`) (`self.Mesh`) false)
  (`SkinnedMeshComponent.SetLeaderPoseComponent` (`self.RightLeg`) (`self.Mesh`) false)
  (`SkinnedMeshComponent.SetLeaderPoseComponent` (`self.RightCalf`) (`self.Mesh`) false)
  (`SkinnedMeshComponent.SetLeaderPoseComponent` (`self.LeftLeg`) (`self.Mesh`) false)
  (`SkinnedMeshComponent.SetLeaderPoseComponent` (`self.LeftCalf`) (`self.Mesh`) false))