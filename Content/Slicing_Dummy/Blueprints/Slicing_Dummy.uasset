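; Dismemberment test dummy whose arms pop off when a BP_Sword overlaps a shoulder collider.
; Construction binds the modular body-part meshes to one master pose mesh.
; SeverLimb hides the arm bones, skipping if already hidden, then spawns a gore-part actor and launches it with a fixed impulse.
; Gate logic for forearm and upper-arm cuts is unfinished: its inputs are unwired, and debug prints remain.
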(event `self.ReceiveBeginPlay`)

(event `CloseLeftArmGate`
  (bind _slicedleftarm (`self.SlicedLeftArm`))
  (bind _forearm_l (`self.Forearm_L`))
  (bind _array (`|MakeArray` (`self.UpperArm_L`) _forearm_l))
  ;[1 1 1] Left Arm Dismemberment
  (`/Engine/EditorBlueprintResources/StandardMacros.Gate` false :!via `Close`
    (:`Exit`
      (if _slicedleftarm
        (if (and (`self.SlicedLeftArm`) (`self.SlicedLeftForearm`))
          (`self.Sever Limb` "/Game/Slicing_Dummy/Blueprints/Slicing_LeftUpperArm.Slicing_LeftUpperArm_C" _array)
          (else
            (`self.Sever Limb` "/Game/Slicing_Dummy/Blueprints/Slicing_LeftArm.Slicing_LeftArm_C" _array)))
        (`self.CloseLeftArmGate`)
        (else
          (if (and (not _slicedleftarm) (`self.SlicedLeftForearm`))
            (`self.Sever Limb` "/Game/Slicing_Dummy/Blueprints/Slicing_LeftForearm.Slicing_LeftForearm_C" (`|MakeArray` _forearm_l))))))))

(event `self.ReceiveTick`
  (params (DeltaSeconds :type "Float (single-precision)")))

(event `CloseRightArmGate`
  (bind _forearm_r (`self.Forearm_R`))
  (bind _slicedrightarm (`self.SlicedRightArm`))
  (bind _array (`|MakeArray` (`self.UpperArm_R`) _forearm_r))
  ;[1 1 1] Right Arm Dismemberment
  (`/Engine/EditorBlueprintResources/StandardMacros.Gate` false :!via `Close`
    (:`Exit`
      (if _slicedrightarm
        (if (and (`self.SlicedRightArm`) (`self.SlicedRightForearm`))
          (`self.Sever Limb` "/Game/Slicing_Dummy/Blueprints/Slicing_LeftUpperArm.Slicing_LeftUpperArm_C" _array)
          (else
            (`self.Sever Limb` "/Game/Slicing_Dummy/Blueprints/Slicing_RightArm.Slicing_RightArm_C" _array)))
        (`self.CloseRightArmGate`)
        (else
          (if (and (not _slicedrightarm) (`self.SlicedRightForearm`))
            (`self.Sever Limb` "/Game/Slicing_Dummy/Blueprints/Slicing_LeftForearm.Slicing_LeftForearm_C" (`|MakeArray` _forearm_r))))))))

(event `self.RightShoulderCollider.OnComponentBeginOverlap`
  (params (OverlappedComponent :type "PrimitiveComponent Object Reference") (OtherActor :type "Actor Object Reference") (OtherComp :type "PrimitiveComponent Object Reference") (OtherBodyIndex :type Integer) (bFromSweep :type Boolean) (SweepResult :type "HitResult Structure (by ref)"))
  (`KismetSystemLibrary.PrintString` "OVERLAP R SHOULDER")
  (cast `/Game/Transfusion/Blueprints/BP_Sword/BP_Sword` (`ActorComponent.GetOwner` OtherComp)
    (:`then`
      (if (`self.SlicedRightArm`)
        (`KismetSystemLibrary.PrintString` "ALREADY SLICED")
        (else
          (`self.Sever Limb` "/Game/Slicing_Dummy/Blueprints/Slicing_RightArm.Slicing_RightArm_C" (`|MakeArray` (`self.UpperArm_R`) (`self.Forearm_R`)))
          (`KismetSystemLibrary.PrintString` "SEVERED LIMB"))))
    (:`CastFailed`
      (`KismetSystemLibrary.PrintString` "FAILED CAST"))))

(event `self.LeftShoulderCollider.OnComponentBeginOverlap`
  (params (OverlappedComponent :type "PrimitiveComponent Object Reference") (OtherActor :type "Actor Object Reference") (OtherComp :type "PrimitiveComponent Object Reference") (OtherBodyIndex :type Integer) (bFromSweep :type Boolean) (SweepResult :type "HitResult Structure (by ref)"))
  (`KismetSystemLibrary.PrintString` "OVERLAP L SHOULDER")
  (cast `/Game/Transfusion/Blueprints/BP_Sword/BP_Sword` (`ActorComponent.GetOwner` OtherComp)
    (:`then`
      (if (`self.SlicedLeftArm`)
        (`KismetSystemLibrary.PrintString` "ALREADY SLICED")
        (else
          (`self.Sever Limb` "/Game/Slicing_Dummy/Blueprints/Slicing_LeftArm.Slicing_LeftArm_C" (`|MakeArray` (`self.UpperArm_L`) (`self.Forearm_L`)))
          (`KismetSystemLibrary.PrintString` "SEVERED LIMB"))))
    (:`CastFailed`
      (`KismetSystemLibrary.PrintString` "FAILED CAST"))))

(fn `Sever Limb`
  (params (GorePart :type "Actor Class Reference") (`Bone(s)` :type "Array of Name"))
  (locals (Skip :type Boolean))
  (bind (_returnvalue_x _returnvalue_y _returnvalue_z) (`KismetMathLibrary.BreakVector` (`SceneComponent.GetSocketLocation` (`self.Mesh`) (`|GetArrayItem` `Bone(s)`))))
  (set `local.Skip` true)
  (for _array_element `Bone(s)`
    (bind _returnvalue (`SkinnedMeshComponent.IsBoneHiddenByName` (`self.Mesh`) _array_element))
    (if (not _returnvalue)
      (set `local.Skip` false)))
  (if (not (`local.Skip`))
    (for _array_element_2 (`local.Bone(s)`)
      (`SkinnedMeshComponent.HideBoneByName` (`self.Mesh`) _array_element_2 "PBO_None"))
    (bind _returnvalue_2 (`|SpawnActorFromClass` (`local.GorePart`) (`KismetMathLibrary.MakeTransform` (`KismetMathLibrary.MakeVector` _returnvalue_x _returnvalue_y (- _returnvalue_z 100.0))) "Undefined" "OverrideRootScale" null null))
    (`PrimitiveComponent.AddImpulse` (`self.GetComponentByClass` _returnvalue_2 "/Script/Engine.SkeletalMeshComponent") (`KismetMathLibrary.MakeVector` 500.0 -500.0 500.0) (`|GetArrayItem` (`local.Bone(s)`)) true)
    (`KismetSystemLibrary.PrintString` (`KismetStringLibrary.Concat_StrStr` "SLICED:: " (`KismetSystemLibrary.GetClassDisplayName` (`local.GorePart`))) true true (struct :`R` 0.008464 :`G` 0.052599 :`B` 0.8125 :`A` 1.0))))

(fn `UserConstructionScript`
  (`SkinnedMeshComponent.SetLeaderPoseComponent` (`self.Torso`) (`self.Mesh`) false)
  (`SkinnedMeshComponent.SetLeaderPoseComponent` (`self.LeftArm`) (`self.Mesh`) false)
  (`SkinnedMeshComponent.SetLeaderPoseComponent` (`self.LeftForearm`) (`self.Mesh`) false)
  (`SkinnedMeshComponent.SetLeaderPoseComponent` (`self.RightArm`) (`self.Mesh`) false)
  (`SkinnedMeshComponent.SetLeaderPoseComponent` (`self.RightForearm`) (`self.Mesh`) false)
  (`SkinnedMeshComponent.SetLeaderPoseComponent` (`self.Pelvis`) (`self.Mesh`) false)
  (`SkinnedMeshComponent.SetLeaderPoseComponent` (`self.RightLeg`) (`self.Mesh`) false)
  (`SkinnedMeshComponent.SetLeaderPoseComponent` (`self.RightCalf`) (`self.Mesh`) false)
  (`SkinnedMeshComponent.SetLeaderPoseComponent` (`self.LeftLeg`) (`self.Mesh`) false)
  (`SkinnedMeshComponent.SetLeaderPoseComponent` (`self.LeftCalf`) (`self.Mesh`) false))