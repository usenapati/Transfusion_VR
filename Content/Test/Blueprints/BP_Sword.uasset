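; BP_Sword is a test VR sword that can be grabbed through a GrabComponent.
; Grab and drop events switch gravity on the sword mesh off and on.
; Disconnected logic would interpolate the held mesh toward the motion controller with a swept teleport, offsetting rotation by the inverted grab rotation, but Tick is empty, so it never runs.
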(event `self.GrabComponent.OnGrabbed`
  (`PrimitiveComponent.SetEnableGravity` (`self.SwordMesh`) false))

(event `self.GrabComponent.OnDropped`
  (`PrimitiveComponent.SetEnableGravity` (`self.SwordMesh`) true))

(event `self.ReceiveTick`
  (params (DeltaSeconds :type "Float (single-precision)")))

(fn `UserConstructionScript`)